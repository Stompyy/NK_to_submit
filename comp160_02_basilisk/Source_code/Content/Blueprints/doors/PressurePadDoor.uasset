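; Sliding double door that opens when the player has entered its room and enough pressure pads are pressed.
; DoorCheck, not called within this Blueprint, counts pressed PressurePad actors level-wide against a required number once the construction-scaled trigger has detected the player.
; Tick slides both halves apart a fixed step per frame to a set distance, updating a spawned arch light's colour.
; Nothing closes the doors or clears the player-in-room flag.
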(event OnComponentBeginOverlap(PlayerInRoomCollider)
  (params (OverlappedComponent :type Primitive%20Component%20Object%20Reference) (OtherActor :type Actor%20Object%20Reference) (OtherComp :type Primitive%20Component%20Object%20Reference) (OtherBodyIndex :type Integer) (bFromSweep :type Boolean) (SweepResult :type Hit%20Result%20Structure%20%28by%20ref%29))
  (if (Actor|ActorHasTag OtherActor "Player")
    (Variables|Default|SetPlayerInRoom true)))

(event Custom|DoorCheck
  (if (Variables|Default|GetPlayerInRoom)
    (bind _outactors (Actor|GetAllActorsOfClass "/Game/Blueprints/doors/PressurePad.PressurePad_C"))
    (for _array_element _outactors
      (if (Variables|/Game/Blueprints/doors/PressurePad.PressurePad_C|GetIsPressed _array_element)
        (bind _result (Math|Integer|IncrementInt (Variables|Default|GetPressurePadsPressed))
          (:%20%20
            (Variables|Default|SetPressurePadsPressed _result)))))
    (if (>= (Variables|Default|GetPressurePadsPressed) (Variables|Default|GetNumberOfPressToOpenDoors))
      (Variables|Default|SetOpenDoors true)
      (else
        (Variables|Default|SetOpenDoors false)))
    (Variables|Default|SetPressurePadsPressed 0)))

(event EventBeginPlay
  (bind _returnvalue (Game|SpawnActorfromClass "/Game/Blueprints/doors/ArchLightBP.ArchLightBP_C" (Transformation|GetWorldTransform (Variables|Default|GetScene)) "Undefined" 0 0))
  (Variables|Default|SetArchLight _returnvalue))

(event EventTick
  (params (DeltaSeconds :type Float%20%28single-precision%29))
  (if (Variables|Default|GetOpenDoors)
    (if (not (Variables|Default|GetDoorsOpen))
      (Transformation|AddLocalOffset (Variables|Default|GetRightDoor) (Math|Vector|MakeVector 0.0 (* (Variables|Default|GetOffsetPerTick) -1.0) 0.0) false false)
      (Transformation|AddLocalOffset (Variables|Default|GetLeftDoor) (Math|Vector|MakeVector 0.0 (Variables|Default|GetOffsetPerTick) 0.0) false false)
      (Variables|Default|SetDistanceMoved (+ (Variables|Default|GetDistanceMoved) (Variables|Default|GetOffsetPerTick)))
      (Variables|Default|SetDoorsOpen (<= 2.5e+02 (Variables|Default|GetDistanceMoved)))
      (Default|EventChangeColour (Variables|Default|GetArchLight)))))

(fn ConstructionScript
  (Class|SceneComponent|AddLocalTransform (Variables|Default|GetPlayerInRoomCollider) (Math|Transform|MakeTransform "0, 0, 0" "0, 0, 0" (Variables|Default|GetSizeOfBox)) false false))