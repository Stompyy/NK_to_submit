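; PvP room door that slides two panels apart once enough players have died while PvP is active.
; A construction-scaled room collider activates PvP when a player overlaps it and gives that player the enemy tag.
; PlayerHasDied counts deaths; at the required total it destroys the collider, ends PvP and strips the tag from all KingArthurController actors.
; Tick then offsets both panels until they reach a fixed travel distance.
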(event OnComponentBeginOverlap(PlayerInRoomCollider)
  (params (OverlappedComponent :type Primitive%20Component%20Object%20Reference) (OtherActor :type Actor%20Object%20Reference) (OtherComp :type Primitive%20Component%20Object%20Reference) (OtherBodyIndex :type Integer) (bFromSweep :type Boolean) (SweepResult :type Hit%20Result%20Structure%20%28by%20ref%29))
  (bind _tags (Variables|/Script/Engine.Actor|GetTags OtherActor))
  (if (Actor|ActorHasTag OtherActor "Player")
    (Variables|Default|SetPvPActive true)
    (Development|PrintString "PVP ACTIVE")
    (Utilities|CheckifPlayerHasEnemyTag _tags _tags)))

(event Custom|PlayerHasDied
  (if (Variables|Default|GetPvPActive)
    (bind _result (Math|Integer|IncrementInt (Variables|Default|GetDeadPlayersDoor))
      (:%20%20
        (if (>= _result (Variables|Default|GetRequiredKillsToOpen))
          (Variables|Default|SetOpenDoors true)
          (Components|DestroyComponent (Variables|Default|GetPlayerInRoomCollider))
          (Variables|Default|SetPvPActive false)
          (bind _outactors (Actor|GetAllActorsOfClass "/Game/Blueprints/ControllerBlueprints/KingArthurController.KingArthurController_C"))
          (for _array_element _outactors
            (Utilities|Array|RemoveItem (Variables|/Script/Engine.Actor|GetTags _array_element) (Variables|Default|GetEnemyTag)))
          (else
            (Variables|Default|SetOpenDoors false)))))))

(event EventTick
  (params (DeltaSeconds :type Float%20%28single-precision%29))
  (if (Variables|Default|GetOpenDoors)
    (if (not (Variables|Default|GetDoorsOpen))
      (Transformation|AddLocalOffset (Variables|Default|GetRightDoor) (Math|Vector|MakeVector 0.0 (* (Variables|Default|GetOffsetPerTick) -1.0) 0.0) false false)
      (Transformation|AddLocalOffset (Variables|Default|GetLeftDoor) (Math|Vector|MakeVector 0.0 (Variables|Default|GetOffsetPerTick) 0.0) false false)
      (Variables|Default|SetDistanceMoved (+ (Variables|Default|GetDistanceMoved) (Variables|Default|GetOffsetPerTick)))
      (Variables|Default|SetDoorsOpen (<= 2.5e+02 (Variables|Default|GetDistanceMoved))))))

(fn ConstructionScript
  (Class|SceneComponent|AddLocalTransform (Variables|Default|GetPlayerInRoomCollider) (Math|Transform|MakeTransform "0, 0, 0" "0, 0, 0" (Variables|Default|GetSizeOfBox)) false false))