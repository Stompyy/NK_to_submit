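; Pressure pad that latches pressed when an actor tagged Player overlaps its box, with no release logic.
; Pressing swaps the mesh from the fire material to the poison material, sets IsPressed and plays a 2D sound.
; It then calls DoorCheck on every PressurePadDoor found in the level, leaving the opening decision to the doors.
; The construction script adds the pad's IndexSelf to PressurePadIndex.
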(event OnComponentBeginOverlap(Box)
  (params (OverlappedComponent :type Primitive%20Component%20Object%20Reference) (OtherActor :type Actor%20Object%20Reference) (OtherComp :type Primitive%20Component%20Object%20Reference) (OtherBodyIndex :type Integer) (bFromSweep :type Boolean) (SweepResult :type Hit%20Result%20Structure%20%28by%20ref%29))
  (if (Actor|ActorHasTag OtherActor "Player")
    (Rendering|Material|SetMaterial (Variables|Default|GetStaticMesh) 0 "/Game/Models/Weapons/Crossbow/CrossBowProjectileMaster_Poison.CrossBowProjectileMaster_Poison")
    (Variables|Default|SetIsPressed true)
    (Audio|PlaySound2D "/Game/Audio/RoomSFX/Pressure_Pad_SFX2.Pressure_Pad_SFX2")
    (bind _outactors (Actor|GetAllActorsOfClass "/Game/Blueprints/Doors/PressurePadDoor.PressurePadDoor_C"))
    (Default|DoorCheck _outactors)))

(event EventBeginPlay
  (Rendering|Material|SetMaterial (Variables|Default|GetStaticMesh) 0 "/Game/Models/Weapons/Crossbow/CrossBowProjectileMaster_Fire.CrossBowProjectileMaster_Fire"))

(event EventTick
  (params (DeltaSeconds :type Float%20%28single-precision%29)))

(fn ConstructionScript
  (Utilities|Array|Add (Variables|Default|GetPressurePadIndex) (Variables|Default|GetIndexSelf)))