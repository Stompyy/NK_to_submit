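; Medium2 is an enemy character that attacks the player on contact and breaks apart on death.
; An overlap with a ParentCharacter while alive starts a looping timer at AttackSpeed rate, playing an animation and sending fixed damage through AffecthealthMessage.
; The death event stops movement, toggles mesh and DestructibleMesh visibility, and applies radial damage to trigger destruction before destroying the actor after a delay.
; The construction script sets default health and walk speed.
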(event EventDamagethePlayer
  ;[1 1 1] attacks the player
  (Components|Animation|PlayAnimation (Variables|Character|GetMesh) 0 false)
  (Class|IDamageable|Affecthealth(Message) (Variables|Default|GetPlayer) 5.0))

(event Collision|EventActorBeginOverlap
  (params (OtherActor :type Actor%20Object%20Reference))
  ;[1 1 1] Finds players in range and calls the attack function
  (if (not (Variables|Default|GetIsDead))
    (bind _asparent_character (Utilities|Casting|CastToParentCharacter OtherActor))
    (Variables|Default|SetPlayer _asparent_character)
    (Utilities|Time|SetTimerbyFunctionName 0 "DamageThePlayer" (/ 1.0 (Variables|Default|GetAttackSpeed)) true)))

(event EventEventDeathEffects
  (bind _destructiblemesh (Variables|Default|GetDestructibleMesh))
  (bind _returnvalue (Transformation|GetWorldLocation _destructiblemesh))
  ;[1 1 1] Repaces mesh witha  destructable mesh and initiates destruction
  (Components|Activation|Activate (Variables|Default|GetSmoke) false)
  (Pawn|Components|CharacterMovement|DisableMovement (Variables|Character|GetCharacterMovement))
  (Components|Activation|Deactivate (Variables|Default|GetSmoke))
  (Rendering|ToggleVisibility (Variables|Default|GetDestructibleMesh) false)
  (Game|Damage|ApplyRadialDamage 1e+03 (Math|Vector|MakeVector (.x _returnvalue) (.y _returnvalue) (+ (.z _returnvalue) (Variables|Default|GetExplosionHeightOffset))) 1e+01 "/Script/Engine.DamageType" 0 0 0 true "ECC_Visibility")
  (Utilities|FlowControl|Delay 1.0)
  (Actor|DestroyActor))

(fn ConstructionScript
  (Variables|Default|Setdefaultwalkspeed 1.0)
  (Variables|Default|SetHealth 1e+02))