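; ParentEnemy is a base enemy Blueprint that handles status effects applied to enemies.
; StatusEffectInfo stores the incoming effect data, then either stuns the enemy by zeroing walk speed for TimeOfStun or starts damage over time.
; Damage over time re-calls StatusEffect each second, sending AffecthealthMessage until the loop count from EffectDuration runs out.
; Stun length ignores EffectDuration, and walk speed restores to the value cached at BeginPlay.
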(event Custom|StatusEffect
  (if (not (<= (Variables|Default|GetEffectLoops) 0))
    (Math|Integer|DecrementInt (Variables|Default|GetEffectLoops)
      (:%20%20
        (Class|IDamageable|Affecthealth(Message) self (Math|Conversions|ToFloat(Integer) (Variables|Default|GetDamageOfEffect)))
        (Utilities|FlowControl|Delay 1.0)
        (CallFunction|StatusEffect)))))

(event EventBeginPlay
  (Variables|Default|Setdefaultwalkspeed (Variables|/Script/Engine.CharacterMovementComponent|GetMaxWalkSpeed (Variables|Character|GetCharacterMovement))))

(event EventStatusEffectInfo
  (params (EffectDuration :type Integer) (EffectDamage :type Integer) (EffectType :type Integer))
  (Variables|Default|SetEffectLoops EffectDuration)
  (Variables|Default|SetDamageOfEffect EffectDamage)
  (bind _output_get (Variables|Default|SetEffectType EffectType))
  (switch int _output_get
    (:1
      (Variables|/Script/Engine.CharacterMovementComponent|SetMaxWalkSpeed (Variables|Character|GetCharacterMovement) 0.0)
      (Utilities|FlowControl|Delay (Variables|Default|GetTimeOfStun))
      (Variables|/Script/Engine.CharacterMovementComponent|SetMaxWalkSpeed (Variables|Character|GetCharacterMovement) (Variables|Default|Getdefaultwalkspeed)))
    (:2
      (CallFunction|StatusEffect))))

(fn ConstructionScript)