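; Grunt enemy that stays immobile until a ParentCharacter enters its one-shot AttackTrigger box, placed per instance by the construction script.
; While the player overlaps Box1, a looping timer deals melee damage at a rate set by AttackSpeed.
; Each hit taken spawns impulse-launched gib chunks and lowers health.
; On death, it swaps its meshes for a destructible, shattered by radial damage with an explosion effect.
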(event OnComponentBeginOverlap(AttackTrigger)
  (params (OverlappedComponent :type Primitive%20Component%20Object%20Reference) (OtherActor :type Actor%20Object%20Reference) (OtherComp :type Primitive%20Component%20Object%20Reference) (OtherBodyIndex :type Integer) (bFromSweep :type Boolean) (SweepResult :type Hit%20Result%20Structure%20%28by%20ref%29))
  (Utilities|Casting|CastToParentCharacter OtherActor)
  ;[1 1 1] Grunt does not move until a player enters the AttackTrigger box
  (Variables|/Script/Engine.CharacterMovementComponent|SetMaxWalkSpeed (Variables|Character|GetCharacterMovement) 6e+02)
  (Components|DestroyComponent (Variables|Default|GetAttackTrigger)))

(event OnComponentBeginOverlap(Box1)
  (params (OverlappedComponent :type Primitive%20Component%20Object%20Reference) (OtherActor :type Actor%20Object%20Reference) (OtherComp :type Primitive%20Component%20Object%20Reference) (OtherBodyIndex :type Integer) (bFromSweep :type Boolean) (SweepResult :type Hit%20Result%20Structure%20%28by%20ref%29))
  (bind _asparent_character (Utilities|Casting|CastToParentCharacter OtherActor))
  (Variables|Default|SetPlayer _asparent_character)
  ;[1 1 1] calls the damage funstion to damage the player
  (Utilities|Time|SetTimerbyFunctionName 0 "DamageThePlayer" (/ 1.0 (Variables|Default|GetAttackSpeed)) true))

(event OnComponentEndOverlap(Box1)
  (params (OverlappedComponent :type Primitive%20Component%20Object%20Reference) (OtherActor :type Actor%20Object%20Reference) (OtherComp :type Primitive%20Component%20Object%20Reference) (OtherBodyIndex :type Integer))
  ;[1 1 1] stops attacking the player when they're out of range
  (if (== OtherActor (Variables|Default|GetPlayer))
    (Utilities|Time|ClearTimerbyFunctionName 0 "DamageThePlayer")))

(event Custom|DamageThePlayer
  ;[1 1 1] Deals damage to the player
  (Variables|Default|SetIsAttacking true)
  (Class|IDamageable|Affecthealth(Message) (Variables|Default|GetPlayer) (Variables|Default|GetAttackDamage))
  (Utilities|FlowControl|Delay 0.6)
  (Variables|Default|SetIsAttacking false))

(event EventBeginPlay
  (Variables|Default|Setdefaultwalkspeed (Variables|/Script/Engine.CharacterMovementComponent|GetMaxWalkSpeed (Variables|Character|GetCharacterMovement)))
  ;[1 1 1] Grunt does not move until a player enters the AttackTrigger box
  (Variables|/Script/Engine.CharacterMovementComponent|SetMaxWalkSpeed (Variables|Character|GetCharacterMovement) 0.0))

(event EventAffecthealth
  (params (DeltaDamage :type Float%20%28single-precision%29) (Player :type Actor%20Object%20Reference))
  ;[1 1 1] Deals damage to the Grunt
  (Utilities|ChunkSpawner
    (:Completed
      (Variables|Default|SetIsHurt true)
      (bind _output_get (Variables|Default|SetHealth (- (Variables|Default|GetHealth) DeltaDamage)))
      (Utilities|FlowControl|Delay 0.2)
      (Variables|Default|SetIsHurt false)
      ;[1 1 1] checks to see if health == 0
      (if (<= _output_get 0.0)
        (Variables|Default|SetIsDead true)
        (if true
          ;[1 1 1] Toggels the destructable mesh
          (Pawn|Components|CharacterMovement|DisableMovement (Variables|Character|GetCharacterMovement))
          (Utilities|FlowControl|Delay 1.0)
          (Rendering|ToggleVisibility (Variables|Default|GetDestructible) false)
          (Components|DestroyComponent (Variables|Character|GetMesh))
          ;[1 1 1] Applies damage to the destructable mesh, and activates explosion
          (Game|Damage|ApplyRadialDamage 1e+03 (Transformation|GetWorldLocation (Variables|Default|GetCapsuleComponent)) 1e+03 "/Script/Engine.DamageType" 0 0 0 false "ECC_Visibility")
          (Components|Activation|Activate (Variables|Default|Getexplode) false))))))

(fn ConstructionScript
  (Variables|Default|SetHealth 7.5e+02)
  (Variables|Default|Setdefaultwalkspeed (Variables|/Script/Engine.CharacterMovementComponent|GetMaxWalkSpeed (Variables|Character|GetCharacterMovement)))
  (Transformation|SetRelativeLocationAndRotation (Variables|Default|GetAttackTrigger) (Variables|Default|GetTriggerBoxLocation) (Variables|Default|GetTriggerBoxRotation) false false))