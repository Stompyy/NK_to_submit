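; Base gamepad player character with twin-stick movement, stamina-costed dash and area shove, melee or ranged weapons, health and points.
; SmoothMovement and SmoothRotation interpolate stick input with drift deadzones, facing movement unless the right stick aims.
; Spawned weapons attach by tag; Tick passes the melee hit window, refills stamina and feeds a world-space health/stamina widget.
; Damage shakes the controller, and death deducts points and notifies PvP doors and the controller.
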(event Custom|Event%20SlowAttackAnim
  (bind _mesh (Variables|Character|GetMesh))
  ;[1 1 1] Interrupt attack anim on overlap
  (if (Variables|Default|GetCanHitWithWeapon)
    (Variables|/Script/Engine.SkeletalMeshComponent|SetGlobalAnimRateScale _mesh (Variables|Default|GetAnimationSlowingSpeed))
    (Utilities|FlowControl|Delay (Variables|Default|GetAnimationSlowingDelay))
    (Variables|/Script/Engine.SkeletalMeshComponent|SetGlobalAnimRateScale _mesh 1.0)))

(event Custom|Event%20Replenish%20Health
  ;[1 1 1] For health pick up effect
  (Variables|Default|SetTempStartHealth (Variables|Default|GetHealth))
  (Variables|Default|SetTempDeltaHealth (- 1e+02 (Variables|Default|GetHealth)))
  ;;[1 1 1] (zero to one) multiplied by temp delta health value
  (bind _health_replenish_rate (Timeline|HealthReplenish Play)
    (:Update
      (Variables|Default|SetHealth (+ (Variables|Default|GetTempStartHealth) (* _health_replenish_rate (Variables|Default|GetTempDeltaHealth)))))))

(event Custom|Event%20Replenish%20Stamina
  ;[1 1 1] Stamina fills over time
  (if (< (Variables|Default|GetStamina) 99.0)
    (Variables|Default|SetStamina (+ (Variables|Default|GetStamina) (Variables|Default|GetStaminaReplenishRatePerFrame)))))

(event EventShoved
  (params (PositionOfPlayer :type Vector))
  ;[1 1 1] Apply Shove
  (Character|LaunchCharacter (* (- (Transformation|GetWorldLocation (Variables|Collision|GetCapsuleComponent)) PositionOfPlayer) (Variables|Default|GetPushPower)) false false))

(event Collision|EventActorBeginOverlap
  (params (OtherActor :type Actor%20Object%20Reference))
  ;[1 1 1] Adds and Removes enemies in range
  (if (Utilities|DoesObjectImplementInterface OtherActor "/Game/Blueprints/Interfaces/ShoveAble.ShoveAble_C")
    (Utilities|Array|Add (Variables|Default|GetShovablesInRange) OtherActor)))

(event EventBeginPlay
  ;[1 1 1] Gives the player invincibility during spawn
  (Variables|Actor|SetbCanBeDamaged false)
  ;[1 1 1] creates the spawning partical effect
  (Utilities|FlowControl|Delay 0.8)
  (Effects|SpawnEmitteratLocation 0 (Transformation|GetWorldLocation (Variables|Default|GetWidget)) "0, 0,0.000000")
  (Utilities|FlowControl|Delay 0.8)
  ;[1 1 1] Makes the players model visible
  (Rendering|SetVisibility (Variables|Character|GetMesh) true false)
  ;[1 1 1] creates the health and stamina widget
  (bind _returnvalue (UserInterface|CreateWidget "/Game/Blueprints/Menus/WorldSpaceHealth.WorldSpaceHealth_C"))
  ;[1 1 1] Enables inputs for the player and removes invincibility
  (Variables|/Script/Engine.CharacterMovementComponent|SetMaxWalkSpeed (Variables|Character|GetCharacterMovement) (Variables|Default|GetWalkingSpeed))
  (Variables|Default|SetCanControl true)
  (Utilities|FlowControl|Delay 2.0)
  (Variables|Actor|SetbCanBeDamaged true))

(event EventAffecthealth
  (params (DeltaDamage :type Float%20%28single-precision%29) (Player :type Actor%20Object%20Reference))
  ;[1 1 1] Deals damage to player
  (if (Variables|Actor|GetbCanBeDamaged)
    (if (> DeltaDamage 999.0)
      (Variables|Default|SetHasFallen true))
    (bind _asking_arthur_controller (Utilities|Casting|CastToKingArthurController (Pawn|GetController)))
    (Default|ControllerShake _asking_arthur_controller)
    (bind _output_get (Variables|Default|SetHealth (- (Variables|Default|GetHealth) DeltaDamage)))
    ;[1 1 1] Checks if the player is dead. If true, it then deducts points
    (if (<= _output_get 0.0)
      (Variables|Default|SetisDead true)
      (Variables|Default|SetIsAttackable false)
      (Utilities|FlowControl|DoOnce false
        (:Completed
          (Variables|Default|SetPoints (- (Variables|Default|GetPoints) (Variables|Default|GetDeathPenalty)))
          (bind _outactors (Actor|GetAllActorsOfClass "/Game/Blueprints/Doors/PvPDoor.PvPDoor_C"))
          (Default|PlayerHasDied _outactors)
          (Utilities|FlowControl|Delay 0.8)
          (Class|PlayersHealth|TransferHealthInfo(Message) (Pawn|GetController) 0.0 (Transformation|GetWorldLocation (Variables|Collision|GetCapsuleComponent))))))))

(event EventTick
  (params (DeltaSeconds :type Float%20%28single-precision%29))
  ;[1 1 1] If attacking, allow weapon overlap to deal damage
  (if (Variables|Default|GetIsAttacking)
    (bind _asmelee_weapon (Utilities|Casting|CastToMeleeWeapon (Variables|Default|GetRealWeapon))
      (:then
        (Variables|/Game/Blueprints/Weapons/MeleeWeapon.MeleeWeapon_C|SetCanAttack _asmelee_weapon (Variables|Default|GetCanHitWithWeapon)))
      (:CastFailed
        _)))
  ;[1 1 1] Checks to see if the attack animation has finished
  (if (Variables|Default|GetAttackAnimationHasEnded)
    (Variables|Default|SetIsAttacking false)
    (Variables|Default|SetAttackAnimationHasEnded false))
  ;[1 1 1] Deals with the health and stamina widgets around the player
  (Transformation|SetWorldRotation (Variables|Default|GetWidget) "90.000000,0.000000,180.000000" false false)
  (UserInterface|SetWidget (Variables|Default|GetWidget) (stale EventBeginPlay _returnvalue))
  (Default|EventHealthEvent (stale EventBeginPlay _returnvalue) (Variables|Default|GetHealth) (Variables|Default|GetMaxHealth) (Variables|Default|GetPlayerWidgetColour))
  (Default|EventStaminaEvent (stale EventBeginPlay _returnvalue) (Variables|Default|GetStamina) (Variables|Default|GetMaxStamina))
  (CallFunction|EventReplenishStamina))

(event EventCalculatePoints
  (params (Points :type Integer))
  ;[1 1 1] PointGain
  (Variables|Default|SetPoints (+ (Variables|Default|GetPoints) (* Points (Math|Float|Truncate (Variables|Default|GetMultiplier)))))
  (Variables|Default|SetMultiplier (+ (Variables|Default|GetMultiplier) 0.1)))

(event EventPickupType
  (params (Weapon :type Actor%20Class%20Reference) (Player :type Actor%20Object%20Reference))
  (bind _tempsword (Variables|Default|GetTempSword))
  ;[1 1 1] Spawns the players weapon
  (Variables|Default|SetWeaponSpawned true)
  (Actor|DestroyActor (Variables|Default|GetRealWeapon))
  (bind _returnvalue (Game|SpawnActorfromClass Weapon (Transformation|GetWorldTransform _tempsword) "Undefined" self 0))
  (bind _output_get (Variables|Default|SetRealWeapon _returnvalue))
  ;[1 1 1] Checks to see if its a melee or ranged weapon
  (if (Actor|ActorHasTag _output_get "MeleeWeapon")
    (Class|Actor|AttachRootComponentto _output_get _tempsword "None" "SnapToTarget" true)
    (else
      (Class|Actor|AttachRootComponentto _output_get (Variables|Default|GetRangedTemp) "None" "SnapToTarget" true)))
  (Utilities|Array|Add (Variables|/Script/Engine.Actor|GetTags _output_get) (Variables|Default|GetPlayerTag))
  (if (Actor|ActorHasTag _output_get "RangedWeapon")
    (Variables|Default|SetIsRangedAttacking true)
    (else
      (Variables|Default|SetIsRangedAttacking false))))

(event Collision|EventActorEndOverlap
  (params (OtherActor :type Actor%20Object%20Reference))
  ;[1 1 1] Adds and Removes enemies in range
  (if (Utilities|DoesObjectImplementInterface OtherActor "/Game/Blueprints/Interfaces/ShoveAble.ShoveAble_C")
    (Utilities|Array|RemoveItem (Variables|Default|GetShovablesInRange) OtherActor)))

(event Input|AxisEvents|InputAxisMoveUp
  (params (AxisValue :type Float%20%28single-precision%29))
  ;[1 1 1] Smooth Movement
  (Utilities|SmoothMovement AxisValue (stale Input|AxisEvents|InputAxisMoveRight AxisValue)))

(event Input|AxisEvents|InputAxisMoveRight
  (params (AxisValue :type Float%20%28single-precision%29))
  ;[1 1 1] Smooth Movement
  (Utilities|SmoothMovement (stale Input|AxisEvents|InputAxisMoveUp AxisValue) AxisValue) ; enters at MoveRight
)

(event Input|AxisEvents|InputAxisLookup
  (params (AxisValue :type Float%20%28single-precision%29))
  ;[1 1 1] Smooth rotation
  (Utilities|SmoothRotation AxisValue (stale Input|AxisEvents|InputAxisLookRight AxisValue)))

(event Input|AxisEvents|InputAxisLookRight
  (params (AxisValue :type Float%20%28single-precision%29))
  ;[1 1 1] Smooth rotation
  (Utilities|SmoothRotation (stale Input|AxisEvents|InputAxisLookup AxisValue) AxisValue))

(event Input|GamepadEvents|GamepadRightTrigger
  (params (Key :type Key%20Structure :default "AnyKey"))
  (bind _realweapon (Variables|Default|GetRealWeapon))
  (bind _realweapon_2 (Variables|Default|GetRealWeapon))
  (bind _returnvalue (Actor|ActorHasTag _realweapon "RangedWeapon"))
  ;[1 1 1] RangedAttack
  (:Pressed
    (if _returnvalue
      (bind _asacrossbow_bp (Utilities|Casting|CastToACrossbowBP _realweapon_2))
      (Default|PullTrigger _asacrossbow_bp)
      (bind _returnvalue_2 (Class|GameplayStatics|GetPlayerControllerID (.AsPlayer%20Controller (Utilities|Casting|CastToPlayerController (Pawn|GetController)))))
      (Class|PlayerControllerID|IDTransfer(Message) _asacrossbow_bp _returnvalue_2)))
  (:Released
    (if _returnvalue
      (bind _asacrossbow_bp_2 (Utilities|Casting|CastToACrossbowBP _realweapon_2))
      (Default|ReleaseTrigger _asacrossbow_bp_2))))

(event Input|GamepadEvents|GamepadFaceButtonRight
  (params (Key :type Key%20Structure :default "AnyKey"))
  ;[1 1 1] Dash
  (:Pressed
    (if (Math|Boolean|ANDBoolean (Variables|Default|GetCanDash) (not (Variables|Default|GetisDead)) (>= (Variables|Default|GetStamina) (Variables|Default|GetDashStaminaCost)))
      (Variables|Default|SetIsDashing false)
      (Variables|Default|SetStamina (- (Variables|Default|GetStamina) (Variables|Default|GetDashStaminaCost)))
      (Character|LaunchCharacter (* (Variables|Default|GetMovementVector) (Variables|Default|GetDashStrength)) false false)
      (Audio|PlaySound2D 0)
      (Variables|Default|SetCanDash false)
      (Utilities|FlowControl|Delay 2.0)
      (Variables|Default|SetIsDashing false)
      (Variables|Default|SetCanDash true))))

(event Input|GamepadEvents|GamepadRightTrigger
  (params (Key :type Key%20Structure :default "AnyKey"))
  ;[1 1 1] Melee Attack
  (:Pressed
    (if (and (Actor|ActorHasTag (Variables|Default|GetRealWeapon) "MeleeWeapon") (not (Variables|Default|GetIsAttacking)))
      (Variables|Default|SetIsAttacking true)
      (Audio|SpawnSound2D 0))))

(event Input|GamepadEvents|GamepadRightShoulder
  (params (Key :type Key%20Structure :default "AnyKey"))
  ;[1 1 1] Melee Attack
  (:Pressed
    (if (and (Actor|ActorHasTag (Variables|Default|GetRealWeapon) "MeleeWeapon") (not (Variables|Default|GetIsAttacking)))
      (Variables|Default|SetIsAttacking true)
      (Audio|SpawnSound2D 0))))

(event Input|GamepadEvents|GamepadRightShoulder
  (params (Key :type Key%20Structure :default "AnyKey"))
  (bind _realweapon (Variables|Default|GetRealWeapon))
  (bind _realweapon_2 (Variables|Default|GetRealWeapon))
  (bind _returnvalue (Actor|ActorHasTag _realweapon "RangedWeapon"))
  ;[1 1 1] RangedAttack
  (:Pressed
    (if _returnvalue
      (bind _asacrossbow_bp (Utilities|Casting|CastToACrossbowBP _realweapon_2))
      (Default|PullTrigger _asacrossbow_bp)
      (bind _returnvalue_2 (Class|GameplayStatics|GetPlayerControllerID (.AsPlayer%20Controller (Utilities|Casting|CastToPlayerController (Pawn|GetController)))))
      (Class|PlayerControllerID|IDTransfer(Message) _asacrossbow_bp _returnvalue_2)))
  (:Released
    (if _returnvalue
      (bind _asacrossbow_bp_2 (Utilities|Casting|CastToACrossbowBP _realweapon_2))
      (Default|ReleaseTrigger _asacrossbow_bp_2))))

(event Input|GamepadEvents|GamepadDPadLeft
  (params (Key :type Key%20Structure :default "AnyKey"))
  ;[1 1 1] Cheat/DevMode
)

(event Input|GamepadEvents|GamepadLeftTrigger
  (params (Key :type Key%20Structure :default "AnyKey"))
  ;[1 1 1] LeftTrigger to Push Actors with Shovable in Range
  (:Pressed
    (if (>= (Variables|Default|GetStamina) (Variables|Default|GetShoveStaminaCost))
      (Variables|Default|SetStamina (- (Variables|Default|GetStamina) (Variables|Default|GetShoveStaminaCost)))
      (for _array_element (Variables|Default|GetShovablesInRange)
        (Class|ShoveAble|Shoved(Message) _array_element (Transformation|GetWorldLocation (Variables|Collision|GetCapsuleComponent)))))))

(event Input|GamepadEvents|GamepadDPadDown
  (params (Key :type Key%20Structure :default "AnyKey"))
  ;[1 1 1] debugs spawn follower - forces it to respawn on a player
  (:Pressed
    (bind _outactors (Actor|GetAllActorsOfClass "/Game/Blueprints/ControllerBlueprints/SpawnFollower.SpawnFollower_C"))
    (for _array_element _outactors
      (Transformation|SetWorldLocation (Variables|Collision|GetCapsuleComponent) (Transformation|GetActorLocation _array_element) false true))))

(fn ConstructionScript)