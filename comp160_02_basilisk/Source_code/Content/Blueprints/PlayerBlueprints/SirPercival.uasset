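; Sir Percival player Blueprint, setting up this knight's stats and identity and handling sword attack animation.
; Construction script loops over top-level ArthurHUD widgets, loading Points from Player 4's last score, maxing health and stamina, and setting Percival's tag with Galahad's widget colour.
; That setup only runs when a HUD exists.
; DontKillMyself clears the WeaponSpawned flag, and PlayAttackAnimation casts RealWeapon to Sword to play its mesh animation once.
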(fn ConstructionScript
  (bind _foundwidgets (Widget|GetAllWidgetsOfClass "/Game/Blueprints/Menus/ArthurHUD.ArthurHUD_C" true))
  (for _array_element _foundwidgets
    (Variables|Default|SetPoints (Variables|/Game/Blueprints/Menus/ArthurHUD.ArthurHUD_C|GetPlayer4LastScore _array_element))
    (Variables|Default|SetHealth (Variables|Default|GetMaxHealth))
    (Variables|Default|SetStamina (Variables|Default|GetMaxStamina))
    (Variables|Default|SetPlayerTag (Variables|Default|GetSirPercivalTag))
    (Variables|Default|SetPlayerWidgetColour (Variables|Default|GetGalahadColour))))