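; FlyingDamage is a short-lived actor that displays a floating damage number.
; On BeginPlay it writes DamageAmount into its text, picks random upward and sideways speeds, and destroys itself after one second.
; Each Tick it sets its rotation from a look-at toward ActorRef and a yaw offset, while MoveComponentTo drifts the root up and sideways and targets ActorRef's rotation.
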(event EventBeginPlay
  (Rendering|Components|TextRender|SetText (Variables|Default|GetDamageValueText) (Utilities|Text|ToText(Float) (Variables|Default|GetDamageAmount) "HalfToEven"))
  (Variables|Default|SetRandomUpSpeed (Math|Random|RandomIntegerinRange 10 20))
  (Variables|Default|SetLeftOrRight (Math|Random|RandomIntegerinRange -10 10))
  (Utilities|FlowControl|Delay 1.0)
  (Actor|DestroyActor))

(event EventTick
  (params (DeltaSeconds :type Float%20%28single-precision%29))
  (bind _returnvalue (Transformation|GetActorLocation))
  (Transformation|SetActorRotation (Math|Rotator|MakeRotator (.roll (Math|Rotator|FindLookatRotation (Transformation|GetActorLocation) (Transformation|GetActorLocation (Variables|Default|GetActorRef)))) 0.0 (Variables|Default|GetRotationOffSetFix)))
  (Components|MoveComponentTo (Variables|Default|GetDefaultSceneRoot) (+ (Math|Vector|MakeVector (.x _returnvalue) (.y _returnvalue) (+ (.z _returnvalue) (Math|Conversions|ToFloat(Integer) (Variables|Default|GetRandomUpSpeed)))) (* (Transformation|GetActorRightVector) (Variables|Default|GetLeftOrRight))) (Transformation|GetActorRotation (Variables|Default|GetActorRef)) false false 0.2 false))

(fn ConstructionScript)