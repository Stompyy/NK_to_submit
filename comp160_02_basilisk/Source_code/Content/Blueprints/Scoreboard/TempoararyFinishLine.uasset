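; Temporary finish-line trigger actor that ends a round by requesting the final scoreboard.
; Each ParentCharacter overlapping the trigger increments PlayerCount, which is compared against the live count of ParentCharacter actors in the level.
; Once all have entered, it calls EventTempGatherScores on the NebulaKnights game mode.
; The construction script scales the trigger volume by FinishLineSize.
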(event OnComponentBeginOverlap(TempFinishLine)
  (params (OverlappedComponent :type Primitive%20Component%20Object%20Reference) (OtherActor :type Actor%20Object%20Reference) (OtherComp :type Primitive%20Component%20Object%20Reference) (OtherBodyIndex :type Integer) (bFromSweep :type Boolean) (SweepResult :type Hit%20Result%20Structure%20%28by%20ref%29))
  ;[1 1 1] When player enters finishing area, update NumberOfPlayersPlaying variable, increment PlayerCount (that has entered finishing area), compare, if equivalent then draw final score board.
  (Utilities|Casting|CastToParentCharacter OtherActor)
  (bind _outactors (Actor|GetAllActorsOfClass "/Game/Blueprints/PlayerBlueprints/ParentCharacter.ParentCharacter_C"))
  (Variables|Default|SetNumberOfPlayersPlaying (Utilities|Array|Length _outactors))
  (bind _result (Math|Integer|IncrementInt (Variables|Default|GetPlayerCount))
    (:%20%20
      (if (>= _result (Variables|Default|GetNumberOfPlayersPlaying))
        (bind _asnebula_knights (Utilities|Casting|CastToNebulaKnights (Game|GetGameMode)))
        (Default|EventTempGatherScores _asnebula_knights)))))

(event EventBeginPlay)

(event Collision|EventActorBeginOverlap
  (params (OtherActor :type Actor%20Object%20Reference)))

(event EventTick
  (params (DeltaSeconds :type Float%20%28single-precision%29)))

(fn ConstructionScript
  (Transformation|SetWorldScale3D (Variables|Default|GetTempFinishLine) (Variables|Default|GetFinishLineSize)))