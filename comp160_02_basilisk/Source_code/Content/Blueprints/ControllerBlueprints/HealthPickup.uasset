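; HealthPickup is a spinning pickup that restores health to a ParentCharacter on contact.
; The construction script gives each pickup a random rotation speed, which Tick applies as yaw to the static mesh.
; A box trigger overlap plays a 2D sound for any ParentCharacter, even at full health.
; Only when health is below maximum does it call the character's EventReplenishHealth and destroy itself.
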(event OnComponentBeginOverlap(BoxTrigger)
  (params (OverlappedComponent :type Primitive%20Component%20Object%20Reference) (OtherActor :type Actor%20Object%20Reference) (OtherComp :type Primitive%20Component%20Object%20Reference) (OtherBodyIndex :type Integer) (bFromSweep :type Boolean) (SweepResult :type Hit%20Result%20Structure%20%28by%20ref%29))
  (bind _asparent_character (Utilities|Casting|CastToParentCharacter OtherActor))
  (Audio|PlaySound2D 0)
  ;[1 1 1] Cannot pick up if already full health
  (if (< (Variables|/Game/Blueprints/PlayerBlueprints/ParentCharacter.ParentCharacter_C|GetHealth _asparent_character) (Variables|Default|GetMaxPlayerHealth))
    ;[1 1 1] Custom event within ParentCharacter class
    (Default|EventReplenishHealth _asparent_character)
    (Actor|DestroyActor)))

(event EventTick
  (params (DeltaSeconds :type Float%20%28single-precision%29))
  (Transformation|AddWorldRotation (Variables|Default|GetStaticMesh) (Math|Rotator|MakeRotator 0.0 0.0 (Variables|Default|GetRotationSpeed)) false false))

(fn ConstructionScript
  ;[1 1 1] Sets a random rotation speed per pickup
  (Variables|Default|SetRotationSpeed (* (Math|Random|RandomFloat) 2.0)))