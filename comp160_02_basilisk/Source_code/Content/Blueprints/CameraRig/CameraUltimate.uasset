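; Camera rig that follows the players' average position and cuts to a slow-motion zoom on a player who has just died.
; Each Tick it sits at the look-at point actor plus a spring-arm-style offset vector, facing the average-position actor.
; ZoomIn slows global time and picks a random preset offset around the last player position.
; A DoOnce-gated timeline lerps the transform there, then restores time and re-arms the gates.
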(event Custom|Event%20Zoom%20In
  (bind _zoomedcameraoffsets (Variables|Default|GetZoomedCameraOffsets))
  (Utilities|FlowControl|DoOnce false
    (:Completed
      ;[1 1 1] Sets time scale at SlowMo value
      (Utilities|Time|SetGlobalTimeDilation (Variables|Default|GetSlowMoSpeed))
      (Variables|Default|SetZoomedCameraFinalPosition (+ (* (Utilities|Array|Get(acopy) _zoomedcameraoffsets (Math|Random|RandomInteger (Utilities|Array|Length _zoomedcameraoffsets))) (Variables|Default|GetZoomedCameraDistance)) (Variables|Default|GetLastPlayerPosition)))
      ;[1 1 1] For the if statement fork in the event Tick
      (Variables|Default|SetZoomIn true))))

(event Custom|Event%20Reset%20Zoom
  (bind _zoomedcameraoffsets (Variables|Default|GetZoomedCameraOffsets))
  (Utilities|FlowControl|Sequence
    (:then_0
      (Utilities|FlowControl|DoOnce false) ; enters at Reset
    )
    (:then_1
      (Utilities|FlowControl|DoOnce false) ; enters at Reset
    )))

(event EventBeginPlay
  ;[1 1 1] Creates the references to the used scene objects
  (bind _outactors (Actor|GetAllActorsOfClass "/Game/Blueprints/CameraRig/AveragePositionOfPlayers_Blueprint.AveragePositionOfPlayers_Blueprint_C"))
  (Variables|Default|SetCamLookAtObject (Utilities|Array|Get(acopy) _outactors))
  (bind _outactors_2 (Actor|GetAllActorsOfClass "/Game/Blueprints/CameraRig/camLookAtPoint_Blueprint.camLookAtPoint_Blueprint_C"))
  (Variables|Default|SetCameraLookAtPoint (Utilities|Array|Get(acopy) _outactors_2)))

(event EventTick
  (params (DeltaSeconds :type Float%20%28single-precision%29))
  (Game|Player|SetViewTargetwithBlend (Game|GetPlayerController 0) (Components|GetOwner (Variables|Default|GetDefaultSceneRoot)) 2e+02 "VTBlend_EaseIn" 0.0 false)
  (Variables|Default|SetCamPositionAtPoint (Transformation|GetWorldLocation (Variables|/Game/Blueprints/CameraRig/camLookAtPoint_Blueprint.camLookAtPoint_Blueprint_C|GetDefaultSceneRoot1 (Variables|Default|GetCameraLookAtPoint))))
  (Variables|Default|SetCamLookAtPoint (Transformation|GetWorldLocation (VehicleSound|GetRootComponent (Variables|Default|GetCamLookAtObject))))
  ;[1 1 1] Zoom in event fork
  (if (Variables|Default|GetZoomIn)
    (Utilities|FlowControl|DoOnce false
      (:Completed
        ;[1 1 1] Zoom in on player that has just died (information is passed in from the player death event, then vectors are calculated in ZoomIn function above), then zoom out
        (bind _cameralerpvalue (Timeline|MoveCameraInPauseThenOut PlayFromStart)
          (:Update
            (Transformation|SetWorldLocationAndRotation (Variables|Default|GetDefaultSceneRoot) (.Location (Math|Transform|BreakTransform (Math|Transform|Lerp(Transform) (Math|Transform|MakeTransform (+ (Variables|Default|GetCamPositionAtPoint) (Variables|Default|GetMyOwnSpringArm)) (Math|Rotator|FindLookatRotation (Transformation|GetWorldLocation (Variables|Default|GetDefaultSceneRoot)) (Variables|Default|GetCamLookAtPoint))) (Math|Transform|MakeTransform (Variables|Default|GetZoomedCameraFinalPosition) (Math|Rotator|FindLookatRotation (Transformation|GetWorldLocation (Variables|Default|GetDefaultSceneRoot)) (Variables|Default|GetLastPlayerPosition))) _cameralerpvalue))) (.Rotation (Math|Transform|BreakTransform (Math|Transform|Lerp(Transform) (Math|Transform|MakeTransform (+ (Variables|Default|GetCamPositionAtPoint) (Variables|Default|GetMyOwnSpringArm)) (Math|Rotator|FindLookatRotation (Transformation|GetWorldLocation (Variables|Default|GetDefaultSceneRoot)) (Variables|Default|GetCamLookAtPoint))) (Math|Transform|MakeTransform (Variables|Default|GetZoomedCameraFinalPosition) (Math|Rotator|FindLookatRotation (Transformation|GetWorldLocation (Variables|Default|GetDefaultSceneRoot)) (Variables|Default|GetLastPlayerPosition))) _cameralerpvalue))) false false))
          (:Finished
            ;[1 1 1] Sets time scale back to normal and resets variables and DoOnce
            (Utilities|Time|SetGlobalTimeDilation 1.0)
            (Variables|Default|SetZoomIn false)
            (CallFunction|EventResetZoom)))))
    (else
      ;[1 1 1] Normal play camera attached to lookAtObject offset by MyOwnSpringArm Vector3, Set to look directly at (lookAtPoint or CamPositionAtPoint) + MyOwnSpringArm offset vector
      (Transformation|SetWorldLocationAndRotation (Variables|Default|GetDefaultSceneRoot) (+ (Variables|Default|GetCamPositionAtPoint) (Variables|Default|GetMyOwnSpringArm)) (Math|Rotator|FindLookatRotation (Transformation|GetWorldLocation (Variables|Default|GetCamera)) (Variables|Default|GetCamLookAtPoint)) false false))))

(fn ConstructionScript)