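; BattleAxe weapon Blueprint that damages and knocks back actors tagged "Enemy" when they begin overlapping it.
; On overlap, the KnockBackMac macro sends the target a normalized away-from-axe vector scaled by KnockBack through an interface message.
; A health message then applies WeaponDamage, passing the axe itself as the Player argument.
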(event Collision|EventActorBeginOverlap
  (params (OtherActor :type Actor%20Object%20Reference))
  (if (Actor|ActorHasTag OtherActor "Enemy")
    (Utilities|KnockBackMac OtherActor)
    (Class|IDamageable|Affecthealth(Message) OtherActor (Variables|Default|GetWeaponDamage) self)))

(fn ConstructionScript)