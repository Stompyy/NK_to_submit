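; NebulaKnights is a game manager actor for local multiplayer with up to four Arthurian knights, handling players, enemy waves and scores.
; BeginPlay creates local players; spawning swaps each pawn for a knight by controller ID, adds a sword, sets the shared camera and updates enemies' player count.
; Despawning restores an InitialPawn and enables respawning.
; Enemy tallies flag doors open at zero, and HUD scores feed a scoreboard widget.
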(event Custom|SpawnPlayers
  (params (PlayerController :type Player%20Controller%20Object%20Reference))
  (bind _returnvalue (Pawn|GetControlledPawn PlayerController))
  ;[1 1 1] Spawn player
  ;[1 1 1] To get spawn position
  (bind _outactors (Actor|GetAllActorsOfClass "/Game/Blueprints/ControllerBlueprints/SpawnFollower.SpawnFollower_C"))
  (bind _returnvalue_2 (Class|GameplayStatics|GetPlayerControllerID PlayerController))
  (Utilities|IsValid _returnvalue
    (:Is%20Valid
      (Actor|DestroyActor _returnvalue)
      (Math|Integer|IncrementInt (Variables|Default|GetPlayingPlayers)
        (:%20%20
          ;[1 1 1] Assign player based on controller
          (switch int _returnvalue_2
            (:0
              (bind _returnvalue_3 (Game|SpawnActorfromClass "/Game/Blueprints/PlayerBlueprints/KingArthur.KingArthur_C" (Transformation|GetActorTransform (Utilities|Array|Get(acopy) _outactors)) "AlwaysSpawn" 0 0))
              (Pawn|Possess PlayerController _returnvalue_3)
              ;[1 1 1] To allow for spawn in time
              (Utilities|FlowControl|Delay 2.0)
              ;[1 1 1] Assign basic weapon
              (Class|Pick2player|PickupType(Message) _returnvalue_3 "/Game/Blueprints/Weapons/StandardSword.StandardSword_C"))
            (:1
              (bind _returnvalue_4 (Game|SpawnActorfromClass "/Game/Blueprints/PlayerBlueprints/SirLancelot.SirLancelot_C" (Transformation|GetActorTransform (Utilities|Array|Get(acopy) _outactors)) "AlwaysSpawn" 0 0))
              (Pawn|Possess PlayerController _returnvalue_4)
              (Utilities|FlowControl|Delay 2.0)
              (Class|Pick2player|PickupType(Message) _returnvalue_4 "/Game/Blueprints/Weapons/StandardSword.StandardSword_C"))
            (:2
              (bind _returnvalue_5 (Game|SpawnActorfromClass "/Game/Blueprints/PlayerBlueprints/SirGawain.SirGawain_C" (Transformation|GetActorTransform (Utilities|Array|Get(acopy) _outactors)) "AlwaysSpawn" 0 0))
              (Pawn|Possess PlayerController _returnvalue_5)
              (Utilities|FlowControl|Delay 2.0)
              (Class|Pick2player|PickupType(Message) _returnvalue_5 "/Game/Blueprints/Weapons/StandardSword.StandardSword_C"))
            (:3
              (bind _returnvalue_6 (Game|SpawnActorfromClass "/Game/Blueprints/PlayerBlueprints/SirPercival.SirPercival_C" (Transformation|GetActorTransform (Utilities|Array|Get(acopy) _outactors)) "AlwaysSpawn" 0 0))
              (Pawn|Possess PlayerController _returnvalue_6)
              (Utilities|FlowControl|Delay 2.0)
              (Class|Pick2player|PickupType(Message) _returnvalue_6 "/Game/Blueprints/Weapons/StandardSword.StandardSword_C")))
          ;[1 1 1] Set camera
          (Game|Player|SetViewTargetwithBlend PlayerController (Variables|Default|GetCameraUltimate) 0.0 "VTBlend_Linear" 0.0 false)
          ;[1 1 1] Update enemy AI player search parameters
          (bind _outactors_2 (Actor|GetAllActorswithTag "Enemy"))
          (for _array_element _outactors_2
            (Class|AmountOfPlayers|CurrentPlayers(Message) _array_element (Variables|Default|GetPlayingPlayers))))))))

(event Custom|Event%20DrawTempScoreBoard
  ;[1 1 1] Seperate function as seperate task, may want to call at different times, i.e. pause menu
  (bind _returnvalue (UserInterface|CreateWidget "/Game/Blueprints/Scoreboard/ScoreBoard.ScoreBoard_C" 0 (Variables|Default|GetPlayerScores)))
  (UserInterface|Viewport|AddtoViewport _returnvalue 0)
  (Utilities|FlowControl|DoOnce false
    (:Completed
      (Audio|PlaySound2D 0 0.6))))

(event Custom|Event%20TempGatherScores
  (bind _playerscores (Variables|Default|GetPlayerScores))
  (bind _foundwidgets (Widget|GetAllWidgetsOfClass "/Game/Blueprints/Menus/ArthurHUD.ArthurHUD_C" true))
  (for (_array_element _array_index) _playerscores
    ;[1 1 1] Rewrite player scores array with the correct current scores
    (Utilities|Array|SetArrayElem _playerscores _array_index (Utilities|Struct|MakePlayerScore (.name _array_element) (Utilities|Array|Get(acopy) (Utilities|Array|MakeArray (Variables|/Game/Blueprints/Menus/ArthurHUD.ArthurHUD_C|GetPlayer1LastScore (Utilities|Array|Get(acopy) _foundwidgets)) (Variables|/Game/Blueprints/Menus/ArthurHUD.ArthurHUD_C|GetPlayer2LastScore (Utilities|Array|Get(acopy) _foundwidgets)) (Variables|/Game/Blueprints/Menus/ArthurHUD.ArthurHUD_C|GetPlayer3LastScore (Utilities|Array|Get(acopy) _foundwidgets)) (Variables|/Game/Blueprints/Menus/ArthurHUD.ArthurHUD_C|GetPlayer4LastScore (Utilities|Array|Get(acopy) _foundwidgets))) _array_index))))
  (CallFunction|EventDrawTempScoreBoard))

(event Custom|DespawnPlayer
  (params (PlayerController :type Player%20Controller%20Object%20Reference))
  (bind _returnvalue (Pawn|GetControlledPawn PlayerController))
  ;[1 1 1] Despawn player
  (Utilities|IsValid _returnvalue
    (:Is%20Valid
      (Actor|DestroyActor _returnvalue)
      (bind _returnvalue_2 (Game|SpawnActorfromClass "/Game/Blueprints/LevelConstructs/InitialPawn.InitialPawn_C" (Transformation|GetActorTransform (Utilities|Array|Get(acopy) (stale Custom|SpawnPlayers _outactors))) "Undefined" 0 0))
      (Pawn|Possess PlayerController _returnvalue_2)
      (Game|Player|SetViewTargetwithBlend (Game|GetPlayerController 0) (Components|GetOwner (Variables|Default|GetCameraUltimate)) 2e+02 "VTBlend_EaseIn" 0.0 false)
      (for _array_element (Utilities|Array|MakeArray (Game|GetPlayerController 0) (Game|GetPlayerController 1) (Game|GetPlayerController 2) (Game|GetPlayerController 3))
        (bind _asking_arthur_controller (Utilities|Casting|CastToKingArthurController _array_element))
        (Variables|/Game/Blueprints/ControllerBlueprints/KingArthurController.KingArthurController_C|SetPlayerCanRespawn _asking_arthur_controller true)))))

(event EventBeginPlay
  ;[1 1 1] Create the player controllers
  (while (<= (Variables|Default|GetNumberOfPlayers) 3)
    (Variables|Default|SetNumberOfPlayers (+ (Variables|Default|GetNumberOfPlayers) 1))
    (Class|GameplayStatics|CreatePlayer -1)))

(event EventEnemyCount
  (params (EnemyCount :type Integer) (EnemyDead :type Boolean))
  ;[1 1 1] Records number of enemies in new spawn wave
  (Variables|Default|SetNumberOfEnemies (+ EnemyCount (Variables|Default|GetNumberOfEnemies)))
  (if EnemyDead
    (bind _output_get (Variables|Default|SetNumberOfEnemies (- (Variables|Default|GetNumberOfEnemies) 1)))
    (if (<= _output_get 0)
      (Variables|Default|SetOpenDoors true))))

(fn ConstructionScript)