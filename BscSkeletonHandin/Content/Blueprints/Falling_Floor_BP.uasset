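; Floor trap that flashes, drops away and then returns when a ParentCharacter overlaps its FloorCollider.
; The construction script caches the mesh's original material, which is restored after a brief swap to a fire material as a warning.
; After a short delay, one timeline animates the mesh's relative Z for the fall, then a second timeline played in reverse raises it back up.
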(event OnComponentBeginOverlap(FloorCollider)
  (params (OverlappedComponent :type Primitive%20Component%20Object%20Reference) (OtherActor :type Actor%20Object%20Reference) (OtherComp :type Primitive%20Component%20Object%20Reference) (OtherBodyIndex :type Integer) (bFromSweep :type Boolean) (SweepResult :type Hit%20Result%20Structure%20%28by%20ref%29))
  (bind _floormesh (Variables|Default|GetFloorMesh))
  ;[1 1 1] Player overlaps
  (Utilities|Casting|CastToParentCharacter OtherActor)
  ;[1 1 1] Flash red
  (Rendering|Material|SetMaterial _floormesh 0 "/Game/Models/Weapons/Crossbow/CrossBowProjectileMaster_Fire.CrossBowProjectileMaster_Fire")
  (Utilities|FlowControl|Delay 0.2)
  (Rendering|Material|SetMaterial _floormesh 0 (Variables|Default|GetOriginalMaterial))
  (Utilities|FlowControl|Delay 0.4)
  ;[1 1 1] Timer event animates the dropping movement
  (bind _floorpositionz (Timeline|FallingFloorOffset PlayFromStart)
    (:Update
      (Transformation|SetRelativeLocation (Variables|Default|GetFloorMesh) (Math|Vector|MakeVector 0.0 0.0 _floorpositionz) false false))
    (:Finished
      ;[1 1 1] And back up again
      (bind _floorpositionz_2 (Timeline|RisingFloorOffset ReverseFromEnd)
        (:Update
          (Transformation|SetRelativeLocation (Variables|Default|GetFloorMesh) (Math|Vector|MakeVector 0.0 0.0 _floorpositionz_2) false false))))))

(event EventBeginPlay)

(event Collision|EventActorBeginOverlap
  (params (OtherActor :type Actor%20Object%20Reference)))

(event EventTick
  (params (DeltaSeconds :type Float%20%28single-precision%29)))

(fn ConstructionScript
  ;[1 1 1] Stores original material, for flashing effect
  (Variables|Default|SetOriginalMaterial (Rendering|Material|GetMaterial (Variables|Default|GetFloorMesh) 0)))