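; Medium2 is an enemy character that attacks the Arthurian knight player characters on contact.
; While alive, overlapping a knight stores it as Player and starts a looping AttackSpeed-based timer that plays an animation and deals damage; Sir Gawain must also be attackable.
; Its death event stops movement, toggles effects and mesh visibility, applies small-radius radial damage at the destructible mesh, then destroys the actor after a delay.
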(event EventDamagethePlayer
  (Components|Animation|PlayAnimation (Variables|Character|GetMesh) 0 false)
  (Class|IDamageable|Affecthealth(Message) (Variables|Default|GetPlayer) 5.0))

(event Collision|EventActorBeginOverlap
  (params (OtherActor :type Actor%20Object%20Reference))
  (if (not (Variables|Default|GetIsDead))
    (bind _asking_arthur (Utilities|Casting|CastToKingArthur OtherActor)
      (:then
        (Variables|Default|SetPlayer _asking_arthur)
        (Utilities|Time|SetTimerbyFunctionName 0 "DamageThePlayer" (/ 1.0 (Variables|Default|GetAttackSpeed)) true :!label _label))
      (:CastFailed
        (bind _assir_lancelot (Utilities|Casting|CastToSirLancelot OtherActor)
          (:then
            (Variables|Default|SetPlayer _assir_lancelot)
            (goto _label))
          (:CastFailed
            (bind _assir_gawain (Utilities|Casting|CastToSirGawain OtherActor)
              (:then
                (Variables|Default|SetPlayer _assir_gawain)
                (if (Variables|/Game/Blueprints/PlayerBlueprints/SirGawain.SirGawain_C|GetIsAttackable _assir_gawain)
                  (goto _label)))
              (:CastFailed
                (bind _assir_percival (Utilities|Casting|CastToSirPercival OtherActor))
                (Variables|Default|SetPlayer _assir_percival)
                (goto _label)))))))))

(event EventEventDeathEffects
  (bind _destructiblemesh (Variables|Default|GetDestructibleMesh))
  (bind _returnvalue (Transformation|GetWorldLocation _destructiblemesh))
  (Components|Activation|Activate (Variables|Default|GetSmoke) false)
  (Pawn|Components|CharacterMovement|DisableMovement (Variables|Character|GetCharacterMovement))
  (Components|Activation|Deactivate (Variables|Default|GetSmoke))
  (Rendering|ToggleVisibility (Variables|Default|GetDestructibleMesh) false)
  (Game|Damage|ApplyRadialDamage 1e+03 (Math|Vector|MakeVector (.x _returnvalue) (.y _returnvalue) (+ (.z _returnvalue) 3e+01)) 1e+01 "/Script/Engine.DamageType" 0 0 0 true "ECC_Visibility")
  (Utilities|FlowControl|Delay 1.0)
  (Actor|DestroyActor))

(fn ConstructionScript
  (Variables|Default|Setdefaultwalkspeed 1.0)
  (Variables|Default|SetHealth 1e+02))