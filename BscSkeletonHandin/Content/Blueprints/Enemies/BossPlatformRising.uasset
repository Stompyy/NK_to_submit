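; Boss platform actor that opens a lid and raises a Grunt enemy out of the platform.
; The LidBack timeline, started on BeginPlay or by EmergeEnemy, slides the lid aside, then destroys it.
; The BaseUp timeline then lifts the base and Grunt2 together.
; When the rise finishes, side components are destroyed and Grunt2 is detached from the platform.
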(event Custom|EmergeEnemy
  (bind _lidoffset (Timeline|LidBack PlayFromStart)
    (:Update
      (Transformation|SetRelativeLocation (Variables|Default|GetLid) (Math|Vector|MakeVector _lidoffset 0.0 (Variables|Default|GetLidZOffset)) false false))
    (:Finished
      (Components|DestroyComponent (Variables|Default|GetLid))
      (bind _baseup (Timeline|BaseUp PlayFromStart)
        (:Update
          (Transformation|SetRelativeLocation (Variables|Default|GetBase) (Math|Vector|MakeVector 0.0 0.0 _baseup) false false))
        (:Finished
          (Components|DestroyComponent (Variables|Default|Getsides))
          (Transformation|DetachFromComponent (Variables|Default|GetGrunt2) "KeepRelative" "KeepRelative" "KeepRelative" true))))))

(event EventBeginPlay
  (bind _lidoffset (Timeline|LidBack PlayFromStart)
    (:Update
      (Transformation|SetRelativeLocation (Variables|Default|GetLid) (Math|Vector|MakeVector _lidoffset 0.0 (Variables|Default|GetLidZOffset)) false false))
    (:Finished
      (Components|DestroyComponent (Variables|Default|GetLid))
      (bind _baseup (Timeline|BaseUp PlayFromStart)
        (:Update
          (Transformation|SetRelativeLocation (Variables|Default|GetBase) (Math|Vector|MakeVector 0.0 0.0 _baseup) false false))
        (:Finished
          (Components|DestroyComponent (Variables|Default|Getsides))
          (Transformation|DetachFromComponent (Variables|Default|GetGrunt2) "KeepRelative" "KeepRelative" "KeepRelative" true))))))

(event Collision|EventActorBeginOverlap
  (params (OtherActor :type Actor%20Object%20Reference)))

(event EventTick
  (params (DeltaSeconds :type Float%20%28single-precision%29)))

(fn ConstructionScript)