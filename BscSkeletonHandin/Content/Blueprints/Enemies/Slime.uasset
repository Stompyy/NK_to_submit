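; Slime enemy character that damages players by contact and randomly picks one of two material and health variants at construction.
; Overlapping a player starts a looping timer that attacks at AttackSpeed until overlap ends.
; Hits flash the material and spawn floating damage text, while a separate event applies knockback.
; Death awards points to the killer's tag-matched pawn, notifies any SlimeDoor, then runs DeathEffects, kept separate for child overrides.
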(event Custom|Event%20DeathEffects
  ;[1 1 1] Seperate to enable override in child medium enemy for sparks and smoke
  (Audio|PlaySound2D 0)
  (Actor|DestroyActor))

(event Custom|Event%20FlashWhenHit
  ;[1 1 1] Simply changes the material, delays, then sets it back to the original.
  (Rendering|Material|SetMaterial (Variables|Character|GetMesh) 0 0)
  (Utilities|FlowControl|Delay 0.4)
  (Rendering|Material|SetMaterial (Variables|Character|GetMesh) 0 (Variables|Default|GetMeshMaterial))
  (Utilities|FlowControl|Delay 0.1))

(event Custom|DamageThePlayer
  (Components|Animation|PlayAnimation (Variables|Character|GetMesh) 0 false)
  (Class|IDamageable|Affecthealth(Message) (Variables|Default|GetPlayer) (Variables|Default|GetAttackDamage)))

(event EventBeginPlay
  (Variables|Default|SetMeshMaterial (Rendering|Material|GetMaterial (Variables|Character|GetMesh) 0)))

(event Collision|EventActorEndOverlap
  (params (OtherActor :type Actor%20Object%20Reference))
  (if (== OtherActor (Variables|Default|GetPlayer))
    (Utilities|Time|ClearTimerbyFunctionName 0 "DamageThePlayer")))

(event EventKnockBackInfo
  (params (VectorForKnockback :type Vector))
  (Character|LaunchCharacter (Math|Vector|MakeVector (.x VectorForKnockback) (.y VectorForKnockback) 0.0) false false))

(event Collision|EventActorBeginOverlap
  (params (OtherActor :type Actor%20Object%20Reference))
  (if (not (Variables|Default|GetIsDead))
    (bind _asparent_character (Utilities|Casting|CastToParentCharacter OtherActor))
    (Variables|Default|SetPlayer _asparent_character)
    (Utilities|Time|SetTimerbyFunctionName 0 "DamageThePlayer" (/ 1.0 (Variables|Default|GetAttackSpeed)) true)))

(event EventAffecthealth
  (params (DeltaDamage :type Float%20%28single-precision%29) (Player :type Actor%20Object%20Reference))
  (bind _self self)
  (CallFunction|EventFlashwhenHit)
  (bind _output_get (Variables|Default|SetHealth (- (Variables|Default|GetHealth) DeltaDamage)))
  (Game|SpawnActorfromClass "/Game/Blueprints/Menus/FlyingDamage.FlyingDamage_C" (Math|Transform|MakeTransform (.location (Transformation|GetWorldTransform (Variables|Default|GetFlyingText))) "0, 0, 0" "1.000000,1.000000,1.000000") "Undefined" _self DeltaDamage _self)
  (if (<= _output_get 0.0)
    (Variables|Default|SetIsDead true)
    (if true
      (bind _aspawn (Utilities|GetPlayerkilling Player))
      (Class|PointGain|CalculatePoints(Message) _aspawn (Variables|Default|GetPoints))
      (bind _outactors (Utilities|CheckforSlimeDoorinLevel)
        (:then
          (Default|EnemyDeadCheck _outactors))
        (:else
          _))
      ;[1 1 1] Seperate to enable override in child medium enemy for sparks and smoke
      (CallFunction|EventDeathEffects))))

(fn ConstructionScript
  (if (> (Math|Random|RandomIntegerinRange 0 5) 2)
    (Rendering|Material|SetMaterial (Variables|Character|GetMesh) 0 0)
    (Variables|Default|SetHealth 1.2e+02)
    (Variables|Default|SetPoints 15)
    (else
      (Rendering|Material|SetMaterial (Variables|Character|GetMesh) 0 0)
      (Variables|Default|SetHealth 3e+01))))