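; Slime enemy AI controller that makes its pawn chase the nearest living player.
; A looping one-second timer calls TrackPlayer, which sends an AIMoveTo toward the actor returned by the ChaseClosest macro.
; The macro gathers pawns of living KingArthurControllers within MinCheckRange into parallel pawn and distance arrays, then picks the minimum distance.
; Those arrays are never cleared here, and a ParentCharacter search branch is left unconnected.
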(event Custom|TrackPlayer
  ;[1 1 1] runs through the track macro
  (bind _nearestenemy (Utilities|ChaseClosest)
    (:Completed
      (AI|AIMoveTo (Pawn|GetControlledPawn) "0, 0, 0" _nearestenemy 5.0 false))))

(event EventBeginPlay
  ;[1 1 1] calls the track player function
  (Utilities|Time|SetTimerbyFunctionName 0 "TrackPlayer" 1.0 true))

(fn ConstructionScript)