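; Grunt2 is an enemy Blueprint that damages the knight player characters on overlap and can be killed for points.
; Overlapping one of four knight classes stores it as Player and starts a looping "DamageThePlayer" timer paced by AttackSpeed, cleared when overlap ends.
; A custom event sends AttackDamage to the player via an interface message.
; Affecthealth reduces Health; at zero it awards points, notifies the first EnemySpawner and destroys the grunt.
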(event Custom|CustomEvent
  (Class|IDamageable|Affecthealth(Message) (Variables|Default|GetPlayer) (Variables|Default|GetAttackDamage)))

(event Collision|EventActorEndOverlap
  (params (OtherActor :type Actor%20Object%20Reference))
  (if (== OtherActor (Variables|Default|GetPlayer))
    (Utilities|Time|ClearTimerbyFunctionName 0 "DamageThePlayer")))

(event Collision|EventActorBeginOverlap
  (params (OtherActor :type Actor%20Object%20Reference))
  (bind _asking_arthur (Utilities|Casting|CastToKingArthur OtherActor)
    (:then
      (Variables|Default|SetPlayer _asking_arthur))
    (:CastFailed
      (bind _assir_lancelot (Utilities|Casting|CastToSirLancelot OtherActor)
        (:then
          (Variables|Default|SetPlayer _assir_lancelot))
        (:CastFailed
          (bind _assir_gawain (Utilities|Casting|CastToSirGawain OtherActor)
            (:then
              (Variables|Default|SetPlayer _assir_gawain))
            (:CastFailed
              (bind _assir_percival (Utilities|Casting|CastToSirPercival OtherActor))
              (Variables|Default|SetPlayer _assir_percival)))))))
  (Utilities|Time|SetTimerbyFunctionName 0 "DamageThePlayer" (/ 1.0 (Variables|Default|GetAttackSpeed)) true))

(event EventAffecthealth
  (params (DeltaDamage :type Float%20%28single-precision%29) (Player :type Actor%20Object%20Reference))
  (bind _output_get (Variables|Default|SetHealth (- (Variables|Default|GetHealth) DeltaDamage)))
  (if (<= _output_get 0.0)
    (Variables|Default|SetIsDead true)
    (if true
      (bind _outactors (Actor|GetAllActorsOfClass "/Game/Blueprints/Enemies/Spawners/TomsLevelSpawners/EnemySpawner.EnemySpawner_C"))
      (Class|PointGain|CalculatePoints(Message) Player (Variables|Default|GetPoints))
      (Class|EnemyCount|EnemyCount(Message) (Utilities|Array|Get(acopy) _outactors) (Variables|Default|GetEnemykill) false)
      (Actor|DestroyActor))))

(fn ConstructionScript)