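; Drone actor that hovers and turns to face the highest-scoring player.
; Tick plays a timeline that bobs the mesh and, while any ParentCharacter exists, triggers the high-scorer search and rotates the root toward that location.
; The search compares KingArthurController scores, takes the leader's pawn location using the array index as player index, and copies it to the first DroneAIController.
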(event Custom|Event%20GetHighScorer
  ;[1 1 1] Sets current high scorer world location
  (bind _outactors (Actor|GetAllActorsOfClass "/Game/Blueprints/ControllerBlueprints/KingArthurController.KingArthurController_C"))
  (for (_array_element _array_index) _outactors
    (if (> (Variables|/Game/Blueprints/ControllerBlueprints/KingArthurController.KingArthurController_C|GetScore _array_element) (Variables|Default|GetHighestScore))
      (Variables|Default|SetHighestScore (Variables|/Game/Blueprints/ControllerBlueprints/KingArthurController.KingArthurController_C|GetScore _array_element))
      (Variables|Default|SetHighScoringPlayerLocation (Transformation|GetWorldLocation (VehicleSound|GetRootComponent (Game|Player|GetPlayerPawn _array_index))))))
  (Variables|Default|SetHighestScore (Variables|Default|GetTempVarHighScoreReset))
  (bind _outactors_2 (Actor|GetAllActorsOfClass "/Game/Blueprints/Drone/DroneAIController.DroneAIController_C"))
  (Variables|/Game/Blueprints/Drone/DroneAIController.DroneAIController_C|SetHighScoringPlayerLocation (Utilities|Array|Get(acopy) _outactors_2) (Variables|Default|GetHighScoringPlayerLocation)))

(event EventBeginPlay
  ;[1 1 1] Initial position
  (Variables|Default|SetHighScoringPlayerLocation (Transformation|GetWorldLocation (Variables|Default|GetDefaultSceneRoot))))

(event EventTick
  (params (DeltaSeconds :type Float%20%28single-precision%29))
  ;[1 1 1] For Mesh bobbing up and down
  (bind _height (Timeline|DroneBobbing Play)
    (:Update
      (Transformation|SetRelativeLocation (Variables|Default|GetDroneMesh) (Math|Vector|MakeVector 0.0 0.0 (+ (* _height (Variables|Default|GetBobHeight)) (Variables|Default|GetHoverHeight))) false false)
      ;[1 1 1] If players are playing
      (bind _outactors (Actor|GetAllActorsOfClass "/Game/Blueprints/PlayerBlueprints/ParentCharacter.ParentCharacter_C"))
      (if (> (Utilities|Array|Length _outactors) 0)
        (CallFunction|EventGetHighScorer)
        ;[1 1 1] Looks at player
        (Transformation|SetWorldRotation (Variables|Default|GetDefaultSceneRoot) (Math|Rotator|FindLookatRotation (Transformation|GetWorldLocation (Variables|Default|GetDefaultSceneRoot)) (Variables|Default|GetHighScoringPlayerLocation)) false false)))))

(fn ConstructionScript)