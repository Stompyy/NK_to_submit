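; CameraTarget is a camera rig actor that records its camera's world transform and tracks whether it is inside a room.
; Tick copies the camera's world rotation and location into ScrollingCamRotation and ScrollingCamLocation.
; Overlaps with actors tagged RoomTrigger set and clear the InRoom flag.
; Local X scrolling, slower inside rooms, is present but disconnected, so the actor does not move itself.
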(event Collision|EventActorEndOverlap
  (params (OtherActor :type Actor%20Object%20Reference))
  (if (Actor|ActorHasTag OtherActor "RoomTrigger")
    (Variables|Default|SetInRoom false)))

(event Collision|EventActorBeginOverlap
  (params (OtherActor :type Actor%20Object%20Reference))
  (if (Actor|ActorHasTag OtherActor "RoomTrigger")
    (Variables|Default|SetInRoom true)))

(event EventTick
  (params (DeltaSeconds :type Float%20%28single-precision%29))
  (bind _camera (Variables|Default|GetCamera))
  (Variables|Default|SetScrollingCamRotation (Transformation|GetWorldRotation _camera))
  (Variables|Default|SetScrollingCamLocation (Transformation|GetWorldLocation _camera)))

(fn ConstructionScript)