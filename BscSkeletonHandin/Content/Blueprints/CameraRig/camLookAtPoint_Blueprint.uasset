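; Camera look-at point actor that follows the average location of all ParentCharacter actors to frame a multiplayer group.
; Each Tick it pushes that average into a fixed-length position history, seeded at BeginPlay, and moves to the history's moving average for smoothing.
; When the farthest character exceeds StandardPlayerDistance from the center, it offsets back in X and up in Z proportionally to the excess, zooming out.
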(event EventBeginPlay
  ;[1 1 1] Initialises position array filling with start point
  (for _index (range 0 (Variables|Default|GetSmoothingAmountNoOfFramesToAverage))
    (Utilities|Array|Add (Variables|Default|GetHistoryOfPostions) (Transformation|GetWorldLocation (Variables|Default|GetDefaultSceneRoot1)))))

(event Collision|EventActorBeginOverlap
  (params (OtherActor :type Actor%20Object%20Reference)))

(event EventTick
  (params (DeltaSeconds :type Float%20%28single-precision%29))
  (bind _historyofpostions (Variables|Default|GetHistoryOfPostions))
  (bind _historyofpostions_2 (Variables|Default|GetHistoryOfPostions))
  (bind _historyofpostions_3 (Variables|Default|GetHistoryOfPostions))
  (bind _playerdistancesfrom_average (Variables|Default|GetPlayerDistancesFrom%20Average))
  (bind _standardplayerdistance (Variables|Default|GetStandardPlayerDistance))
  (bind _returnvalue (Utilities|Array|Length _historyofpostions_2))
  (bind _maxvalue (Math|Float|MaxOfFloatArray _playerdistancesfrom_average))
  (bind _returnvalue_2 (Math|Vector|GetVectorArrayAverage _historyofpostions))
  (bind _returnvalue_3 (- _maxvalue _standardplayerdistance))
  (bind _returnvalue_4 (* _returnvalue_3 1.5))
  ;[1 1 1] If any players are playing
  (bind _outactors (Actor|GetAllActorsOfClass "/Game/Blueprints/PlayerBlueprints/ParentCharacter.ParentCharacter_C"))
  (if (> (Utilities|Array|Length _outactors) 0)
    (bind _returnvalue_5 (Class|GameplayStatics|GetActorArrayAverageLocation _outactors))
    ;[1 1 1] Returns array of distances from average player position
    (for _array_element _outactors
      (Utilities|Array|Add (Variables|Default|GetPlayerDistancesFrom%20Average) (Math|Vector|VectorLength (- (Transformation|GetWorldLocation (VehicleSound|GetRootComponent _array_element)) _returnvalue_5))))
    ;[1 1 1] Shifts array indexes down one then updates with the latest (moving point average)
    (for _index (range 0 (- _returnvalue 2))
      (Utilities|Array|SetArrayElem _historyofpostions_3 _index (Utilities|Array|Get(acopy) _historyofpostions_3 (+ _index 1))))
    (Utilities|Array|SetArrayElem _historyofpostions_3 (- _returnvalue 1) _returnvalue_5)
    ;[1 1 1] Check greatest player distance from average position, against tolerences, to determine camera action - panning in or out
    (if (> _maxvalue _standardplayerdistance)
      ;[1 1 1] Modified camera height
      (Variables|Default|SetTempPosX (- (.x _returnvalue_2) _returnvalue_4))
      (Variables|Default|SetTempPosZ (+ _returnvalue_4 (.z _returnvalue_2)))
      (else
        ;[1 1 1] Standard camera height
        (Variables|Default|SetTempPosX (.x _returnvalue_2))
        (Variables|Default|SetTempPosZ (.z _returnvalue_2))))
    ;[1 1 1] Using temporary variables to pan camera in and out
    (Transformation|SetWorldLocation (Variables|Default|GetDefaultSceneRoot1) (Math|Vector|MakeVector (Variables|Default|GetTempPosX) (.y (Math|Vector|GetVectorArrayAverage (Variables|Default|GetHistoryOfPostions))) (Variables|Default|GetTempPosZ)) false false)
    ;[1 1 1] Clears temporary array
    (Utilities|Array|Clear (Variables|Default|GetPlayerDistancesFrom%20Average))))

(fn ConstructionScript
  (Variables|Default|SetSmoothingAmountNoOfFramesToAverage (Variables|Default|GetSmoothingAmountNoOfFramesToAverage)))