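; Camera rig that follows the CamLookAtPoint actor and performs slow-motion zoom-ins.
; Normally, Tick holds the camera at a manual spring-arm offset, aimed at that actor, and stores the transform.
; ZoomIn slows global time, raises its own dilation, then lerps per frame toward the look-at point, aiming at a randomly offset player position.
; ZoomOut restores global time and resumes following without blending.
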(event Custom|Event%20Zoom%20In
  ;[1 1 1] Not so temp...
  ;;[1 1 1] Temp event call for zoom in
  (bind _outactors (Actor|GetAllActorsOfClass "/Game/Blueprints/ControllerBlueprints/KingArthurController.KingArthurController_C"))
  (Variables|Default|SetlastPlayerPos (Transformation|GetWorldLocation (VehicleSound|GetRootComponent (Game|Player|GetPlayerPawn 0))))
  (Utilities|Time|SetGlobalTimeDilation 0.1)
  (Variables|Default|SetCustomTimeDilation 1e+02)
  (Utilities|FlowControl|DoOnce false
    (:Completed
      ;[1 1 1] pass in actor to look at
      (Variables|Default|SetpawnToLookAt (Game|Player|GetPlayerPawn 0))
      (Variables|Default|SetzoomedCamFinalPosition (+ (* (Utilities|Array|Get(acopy) (Variables|Default|GetZoomCameraOffsets) (Math|Random|RandomInteger (Utilities|Array|Length (Variables|Default|GetZoomCameraOffsets)))) (Variables|Default|GetzoomCamDistance)) (Variables|Default|GetlastPlayerPos)))
      (Variables|Default|SetzoomIn true)
      (Variables|Default|SetzoomLerp 0.0))))

(event Custom|Event%20Zoom%20Out
  ;[1 1 1] Not so temp...
  ;;[1 1 1] Temp event call for zoom in
  (Utilities|Time|SetGlobalTimeDilation 1.0)
  (Variables|Default|SetzoomIn false)
  (Utilities|FlowControl|DoOnce false) ; enters at Reset
)

(event EventTick
  (params (DeltaSeconds :type Float%20%28single-precision%29))
  (if (Variables|Default|GetzoomIn)
    ;[1 1 1] Lerps zoom in var 0.0 - 1.0
    (if (>= (Variables|Default|GetzoomLerp) 1.0)
      (Variables|Default|SetzoomLerp 1.0)
      (else
        (Variables|Default|SetzoomLerp (+ (Variables|Default|GetzoomLerp) (/ 1.0 (Variables|Default|GetzoomTimeIn))))))
    (Transformation|SetWorldLocationAndRotation (Variables|Default|GetcameraUsedToZoom) (.Location (Math|Transform|BreakTransform (Math|Transform|Lerp(Transform) (Math|Transform|MakeTransform (Variables|Default|GetLastStdCamPosition) (Variables|Default|GetLastStdCamRotation)) (Math|Transform|MakeTransform (Transformation|GetWorldLocation (Variables|/Game/Blueprints/ControllerBlueprints/camLookAtPoint_Blueprint.camLookAtPoint_Blueprint_C|GetDefaultSceneRoot1 (Variables|Default|GetLookAtPointRef))) (Math|Rotator|FindLookatRotation (Transformation|GetWorldLocation (Variables|Default|GetcameraUsedToZoom)) (Variables|Default|GetzoomedCamFinalPosition))) (Variables|Default|GetzoomLerp)))) (.Rotation (Math|Transform|BreakTransform (Math|Transform|Lerp(Transform) (Math|Transform|MakeTransform (Variables|Default|GetLastStdCamPosition) (Variables|Default|GetLastStdCamRotation)) (Math|Transform|MakeTransform (Transformation|GetWorldLocation (Variables|/Game/Blueprints/ControllerBlueprints/camLookAtPoint_Blueprint.camLookAtPoint_Blueprint_C|GetDefaultSceneRoot1 (Variables|Default|GetLookAtPointRef))) (Math|Rotator|FindLookatRotation (Transformation|GetWorldLocation (Variables|Default|GetcameraUsedToZoom)) (Variables|Default|GetzoomedCamFinalPosition))) (Variables|Default|GetzoomLerp)))) false false)
    (else
      (bind _outactors (Actor|GetAllActorsOfClass "/Game/Blueprints/ControllerBlueprints/camLookAtPoint_Blueprint.camLookAtPoint_Blueprint_C"))
      (Variables|Default|SetLookAtPointRef (Utilities|Array|Get(acopy) _outactors))
      (bind _outactors_2 (Actor|GetAllActorsOfClass "/Game/Blueprints/CameraRig/CameraTarget.CameraTarget_C"))
      (Transformation|SetWorldLocationAndRotation (Variables|Default|GetcameraUsedToZoom) (+ (Variables|Default|GetMyOwnSpringArm) (Transformation|GetWorldLocation (Variables|/Game/Blueprints/ControllerBlueprints/camLookAtPoint_Blueprint.camLookAtPoint_Blueprint_C|GetDefaultSceneRoot1 (Utilities|Array|Get(acopy) _outactors)))) (Math|Rotator|FindLookatRotation (Transformation|GetWorldLocation (Variables|Default|GetcameraUsedToZoom)) (Transformation|GetWorldLocation (Variables|/Game/Blueprints/ControllerBlueprints/camLookAtPoint_Blueprint.camLookAtPoint_Blueprint_C|GetDefaultSceneRoot1 (Utilities|Array|Get(acopy) _outactors)))) false false)
      ;[1 1 1] Storing last position for start of zoom in lerp function above
      (Variables|Default|SetLastStdCamPosition (+ (Variables|Default|GetMyOwnSpringArm) (Transformation|GetWorldLocation (Variables|/Game/Blueprints/ControllerBlueprints/camLookAtPoint_Blueprint.camLookAtPoint_Blueprint_C|GetDefaultSceneRoot1 (Utilities|Array|Get(acopy) _outactors)))))
      (Variables|Default|SetLastStdCamRotation (Math|Rotator|FindLookatRotation (Transformation|GetWorldLocation (Variables|Default|GetcameraUsedToZoom)) (Transformation|GetWorldLocation (Variables|/Game/Blueprints/ControllerBlueprints/camLookAtPoint_Blueprint.camLookAtPoint_Blueprint_C|GetDefaultSceneRoot1 (Utilities|Array|Get(acopy) _outactors))))))))

(fn ConstructionScript)