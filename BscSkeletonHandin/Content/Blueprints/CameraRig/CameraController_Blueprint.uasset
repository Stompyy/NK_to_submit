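; Auto-scrolling camera rig actor that moves along its local X axis every tick, slowing while it overlaps an actor tagged RoomTrigger.
; Tick also caches the player's last non-zero position, since it reads zero on death.
; An unfinished zoom picks a random preset offset around that position and lerps the mesh toward it.
; The lerp branch is hard-wired false and the ZoomIn event is empty, so only scrolling moves the camera.
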(event Custom|Event%20Zoom%20In
  ;[1 1 1] Temp event call for zoom in
)

(event Custom|Event%20Zoom%20Out
  (bind _returnvalue (VehicleSound|GetRootComponent))
  (bind _returnvalue_2 (Transformation|GetWorldTransform _returnvalue))
  (bind (_location _rotation) (Math|Transform|BreakTransform _returnvalue_2))
  ;[1 1 1] Temp event call for zoom in
  (Variables|Default|SetzoomIn false)
  (Utilities|FlowControl|DoOnce false ; enters at Reset
    (:Completed
      ;[1 1 1] pass in actor to look at
      (Variables|Default|SetpawnToLookAt (Game|Player|GetPlayerPawn 0))
      (Variables|Default|SetzoomedCamFinalPosition (+ (* (Utilities|Array|Get(acopy) (Variables|Default|GetdeltaZoomCamPosChoices) (Math|Random|RandomInteger (Utilities|Array|Length (Variables|Default|GetdeltaZoomCamPosChoices)))) (Variables|Default|GetzoomCamDistance)) (Variables|Default|GetlastPlayerPos)))
      (Variables|Default|SetzoomIn true)
      (Variables|Default|SetpreviousCamPos _location)
      (Variables|Default|SetpreviousCamRot _rotation))))

(event Collision|EventActorEndOverlap
  (params (OtherActor :type Actor%20Object%20Reference))
  (if (Actor|ActorHasTag OtherActor "RoomTrigger")
    (Variables|Default|SetInRoom false)))

(event Collision|EventActorBeginOverlap
  (params (OtherActor :type Actor%20Object%20Reference))
  (if (Actor|ActorHasTag OtherActor "RoomTrigger")
    (Variables|Default|SetInRoom true)))

(event EventTick
  (params (DeltaSeconds :type Float%20%28single-precision%29))
  (bind _returnvalue (Game|Player|GetPlayerPawn 0))
  (bind _returnvalue_2 (VehicleSound|GetRootComponent _returnvalue))
  (bind _returnvalue_3 (Transformation|GetWorldLocation _returnvalue_2))
  ;[1 1 1] Updates last player pos (as player pos is zero on death)
  (if (Math|Vector|NotEqual(Vector) _returnvalue_3 "0, 0, 0" 0.1)
    (Variables|Default|SetlastPlayerPos _returnvalue_3))
  (if false
    ;[1 1 1] Lerps zoom in var 0.0 - 1.0
    (if (>= (Variables|Default|GetzoomLerp) 1.0)
      (Variables|Default|SetzoomLerp 1.0)
      (else
        (Variables|Default|SetzoomLerp (+ (Variables|Default|GetzoomLerp) (/ 1.0 (Variables|Default|GetzoomTimeIn))))))
    (Transformation|SetWorldLocationAndRotation (Variables|Debug|GetStaticMeshComponent) (.Location (Math|Transform|BreakTransform (Math|Transform|Lerp(Transform) (Math|Transform|MakeTransform (Variables|Default|GetpreviousCamPos) (Variables|Default|GetpreviousCamRot)) (Math|Transform|MakeTransform (Variables|Default|GetzoomedCamFinalPosition) (Math|Rotator|FindLookatRotation (Variables|Default|GetpreviousCamPos) (Variables|Default|GetzoomedCamFinalPosition))) (Variables|Default|GetzoomLerp)))) (.Rotation (Math|Transform|BreakTransform (Math|Transform|Lerp(Transform) (Math|Transform|MakeTransform (Variables|Default|GetpreviousCamPos) (Variables|Default|GetpreviousCamRot)) (Math|Transform|MakeTransform (Variables|Default|GetzoomedCamFinalPosition) (Math|Rotator|FindLookatRotation (Variables|Default|GetpreviousCamPos) (Variables|Default|GetzoomedCamFinalPosition))) (Variables|Default|GetzoomLerp)))) false false)
    (else
      ;[1 1 1] Standard room scroll
      (if (Variables|Default|GetInRoom)
        (Transformation|AddActorLocalOffset (Math|Vector|MakeVector (* DeltaSeconds 5e+01) 0.0 0.0) false true)
        (else
          (Transformation|AddActorLocalOffset (Math|Vector|MakeVector (* DeltaSeconds 1.5e+02) 0.0 0.0) false true))))))

(fn ConstructionScript)