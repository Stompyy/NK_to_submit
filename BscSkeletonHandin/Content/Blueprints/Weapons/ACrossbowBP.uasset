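; Crossbow weapon Blueprint that automatically fires bolt projectiles while the trigger is held.
; PullTrigger passes a DoOnce gate to fire immediately and start a looping Fire timer based on RateOfFire, which ReleaseTrigger clears after a short delay before resetting the gate.
; Fire plays Shot2 and spawns BoltToFire, set to CrossbowProjectile in construction, at ProjectileSpawn using only its yaw and roll, without pitch.
; A custom event stores a ControllerID.
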(event Custom|PullTrigger
  (Utilities|FlowControl|DoOnce false
    (:Completed
      (CallFunction|Fire)
      (Utilities|Time|SetTimerbyFunctionName self "Fire" (/ 1.0 (Variables|Default|GetRateOfFire)) true))))

(event Custom|Fire
  (bind _projectilespawn (Variables|Default|GetProjectileSpawn))
  (bind _returnvalue (Transformation|GetWorldTransform _projectilespawn))
  (Audio|Components|Audio|Play (Variables|Default|GetShot2) 0.0)
  ;[1 1 1] Fires A projectile
  ;;[1 1 1] v
  (Game|SpawnActorfromClass (Variables|Default|GetBoltToFire) (Math|Transform|MakeTransform (.location _returnvalue) (Math|Rotator|MakeRotator (.roll (.rotation _returnvalue)) 0.0 (.yaw (.rotation _returnvalue))) (.scale _returnvalue)) "Undefined" (Components|GetOwner) 0)
  (Utilities|FlowControl|Delay 0.1))

(event Custom|ReleaseTrigger
  (Utilities|FlowControl|Delay 0.5)
  (Utilities|Time|ClearTimerbyFunctionName 0 "Fire")
  (Utilities|FlowControl|DoOnce false) ; enters at Reset
)

(event Custom|CustomEvent
  (params (ControllerID :type Integer))
  (Variables|Default|SetControllerID ControllerID))

(fn ConstructionScript
  (Variables|Default|SetBoltToFire "/Game/Blueprints/Weapons/Projectiles/CrossbowProjectile.CrossbowProjectile_C"))