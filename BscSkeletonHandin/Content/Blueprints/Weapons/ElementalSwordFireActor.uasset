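; Fire elemental sword weapon, a child of a melee parent, that defines its stats through inherited variables.
; The Construction Script sets damage range, knockback and a chance-based damaging status effect with a duration.
; The Event Graph holds only an empty overlap event and disconnected logic for slowing and resetting knight attack animations, implemented only for KingArthur.
; The KnockBackMac macro sends a direction away from the sword scaled by zero.
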(event Collision|EventActorEndOverlap
  (params (OtherActor :type Actor%20Object%20Reference)))

(fn ConstructionScript
  ;[1 1 1] Setting the variables inherited from melee parent. This determines the propperties of the weapon
  (Variables|Default|SetMinWeaponDmg 60)
  (Variables|Default|SetMaxWeaponDmg 70)
  (Variables|Default|SetKnockBack 6e+03)
  (Variables|Default|SetStatusEffectProbability 0.5)
  (Variables|Default|SetEffectType 2)
  (Variables|Default|SetEffectDamage 20)
  (Variables|Default|SetEffectDuration 5))