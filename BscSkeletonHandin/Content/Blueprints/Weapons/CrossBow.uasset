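; Crossbow weapon Blueprint that spawns crossbow projectiles in response to trigger events.
; A trigger pull passes a DoOnce gate, waits briefly, fires, then sets a timer on Fire based on RateOfFire.
; Releasing the trigger clears that timer and resets the gate.
; Fire spawns the projectile at the ProjectileSpawn transform and hands it the ControllerID received through IDTransfer.
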(event Custom|PullTrigger
  (Utilities|FlowControl|DoOnce false
    (:Completed
      (Utilities|FlowControl|Delay 0.3)
      (CallFunction|Fire)
      (Utilities|Time|SetTimerbyFunctionName 0 "Fire" (/ 1.0 (Variables|Default|GetRateOfFire))))))

(event Custom|Fire
  ;[1 1 1] Fires A projectile
  (bind _returnvalue (Game|SpawnActorfromClass "/Game/Blueprints/Weapons/Projectiles/CrossbowProjectile.CrossbowProjectile_C" (Transformation|GetWorldTransform (Variables|Default|GetProjectileSpawn)) "Undefined" 0 0))
  (Class|PlayerControllerID|IDTransfer(Message) _returnvalue (Variables|Default|GetController%20ID)))

(event Custom|ReleaseTrigger
  (Utilities|Time|ClearTimerbyFunctionName 0 "Fire")
  (Utilities|FlowControl|DoOnce false) ; enters at Reset
)

(event EventIDTransfer
  (params (ControllerID :type Integer))
  (Variables|Default|SetController%20ID ControllerID))

(fn ConstructionScript)