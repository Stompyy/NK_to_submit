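; Base melee weapon that, while CanAttack is set, hits overlapped actors with knockback, damage and possible status effects.
; An overlap first slows King Arthur's or pauses another knight's attack animation, finding the pawn by the weapon's second tag.
; It then pushes the target away from the weapon.
; ParentEnemy targets receive random ranged damage and a probability-rolled effect, whose type is meant to be set per weapon.
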(event Collision|EventActorBeginOverlap
  (params (OtherActor :type Actor%20Object%20Reference))
  (if (Variables|Default|GetCanAttack)
    (Utilities|PauseSlowAnimationonOverlap
      (:OutputPin
        (Utilities|KnockBackMac OtherActor)
        ;[1 1 1] Applies damage(in random range) to the target if they inherit from Parent Enemy class
        (bind _asparent_enemy (Utilities|Casting|CastToParentEnemy OtherActor))
        (Class|IDamageable|Affecthealth(Message) _asparent_enemy (Math|Conversions|ToFloat(Integer) (Math|Random|RandomIntegerinRange (Variables|Default|GetMinWeaponDmg) (Variables|Default|GetMaxWeaponDmg))) self)
        ;[1 1 1] May apply status effect dependent on probability, type of status effect is dependent on the weapon and is selected in the construction script of each weapon.
        (if (> (Variables|Default|GetStatusEffectProbability) (Math|Random|RandomFloat))
          (Class|StatusEffect|StatusEffectInfo(Message) _asparent_enemy (Variables|Default|GetEffectDuration) (Variables|Default|GetEffectDamage) (Variables|Default|GetEffectType)))))))

(fn ConstructionScript)