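; Sir Gawain player character: picks up weapons, fights, scores points with a growing multiplier and takes damage.
; Right trigger fires a crossbow or starts a melee attack, with Tick passing the animation-driven hit window to the weapon.
; Damage shakes the controller; death deducts points once and notifies PvP doors and the controller.
; Spawning plays a light-beam intro with brief invulnerability, while Tick feeds health and stamina to a world-space widget.
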(event Custom|Event%20PauseAttackAnim
  (bind _mesh (Variables|Character|GetMesh))
  (if (Variables|Default|GetCanHitWithWeapon)
    (Variables|/Script/Engine.SkeletalMeshComponent|SetGlobalAnimRateScale _mesh (Variables|Default|GetAnimationSlowingSpeed))
    (Utilities|FlowControl|Delay (Variables|Default|GetAnimationSlowingDelay))
    (Variables|/Script/Engine.SkeletalMeshComponent|SetGlobalAnimRateScale _mesh 1.0)))

(event EventBeginPlay
  (Variables|Default|SetbCanBeDamaged false)
  (Utilities|FlowControl|Delay 0.8)
  (Effects|SpawnEmitteratLocation "/Game/TopDownBP/Particles/BiFrost/BeamOfLightP_3.BeamOfLightP_3" (Transformation|GetWorldLocation (Variables|Default|GetWidget)))
  (Audio|PlaySound2D "/Game/Audio/ParticleSFX/character_phase_in_demo.character_phase_in_demo")
  (Utilities|FlowControl|Delay 0.8)
  (Audio|PlaySound2D "/Game/Audio/KnightSFX/Sir_Gawain.Sir_Gawain")
  (Rendering|SetVisibility (Variables|Character|GetMesh) true false)
  (bind _returnvalue (UserInterface|CreateWidget "/Game/Blueprints/Menus/WorldSpaceHealth.WorldSpaceHealth_C"))
  (Variables|/Script/Engine.CharacterMovementComponent|SetMaxWalkSpeed (Variables|Character|GetCharacterMovement) (Variables|Default|GetWalkingSpeed))
  (Variables|Default|SetCanControl true)
  (Utilities|FlowControl|Delay 2.0)
  (Variables|Default|SetbCanBeDamaged true))

(event EventPickupType
  (params (Weapon :type Actor%20Class%20Reference) (Player :type Actor%20Object%20Reference))
  (bind _swordtemp (Variables|Default|GetSwordTemp))
  ;[1 1 1] Attaches the Sword
  (Variables|Default|SetWeaponSpawned true)
  (Actor|DestroyActor (Variables|Default|GetRealWeapon))
  (bind _returnvalue (Game|SpawnActorfromClass Weapon (Transformation|GetWorldTransform _swordtemp) "Undefined" self 0))
  (bind _output_get (Variables|Default|SetRealWeapon _returnvalue))
  (Class|Actor|AttachRootComponentto _output_get _swordtemp "None" "SnapToTarget" true)
  (Utilities|Array|Add (Variables|/Script/Engine.Actor|GetTags _output_get) (Variables|Default|GetSirGawain)))

(event EventAffecthealth
  (params (DeltaDamage :type Float%20%28single-precision%29) (Player :type Actor%20Object%20Reference))
  ;[1 1 1] DealsDamage
  (if (Variables|Default|GetbCanBeDamaged)
    (Utilities|DontKillMyself
      (:else
        (if (not (Actor|ActorHasTag Player (Variables|Default|GetSirGawain)))
          (if (> DeltaDamage 999.0)
            (Variables|Default|SetHasFallen true))
          (bind _asking_arthur_controller (Utilities|Casting|CastToKingArthurController (Pawn|GetController)))
          (Default|ControllerShake _asking_arthur_controller)
          (bind _output_get (Variables|Default|SetHealth (- (Variables|Default|GetHealth) DeltaDamage)))
          (if (<= _output_get 0.0)
            (Variables|Default|SetisDead true)
            (Variables|Default|SetIsAttackable false)
            (Utilities|FlowControl|DoOnce false
              (:Completed
                (Variables|Default|SetPoints (- (Variables|Default|GetPoints) (Variables|Default|GetDeathPenalty)))
                (Utilities|FlowControl|Delay 0.4)
                (bind _outactors (Actor|GetAllActorsOfClass "/Game/Blueprints/Doors/PvPDoor.PvPDoor_C"))
                (Default|PlayerHasDied _outactors)
                (Class|PlayersHealth|TransferHealthInfo(Message) (Pawn|GetController) 0.0 (Transformation|GetWorldLocation (Variables|Default|GetCapsuleComponent)))
                (Development|PrintString "Hello")))))))))

(event EventTick
  (params (DeltaSeconds :type Float%20%28single-precision%29))
  ;[1 1 1] If attacking, allow weapon overlap to deal damage
  (if (Variables|Default|GetIsAttacking)
    (bind _asmelee_weapon (Utilities|Casting|CastToMeleeWeapon (Variables|Default|GetRealWeapon))
      (:then
        (Variables|/Game/Blueprints/Weapons/MeleeWeapon.MeleeWeapon_C|SetCanAttack _asmelee_weapon (Variables|Default|GetCanHitWithWeapon)))
      (:CastFailed
        _)))
  (if (Variables|Default|GetAttackAnimationHasEnded)
    (Variables|Default|SetIsAttacking false)
    (Variables|Default|SetAttackAnimationHasEnded false))
  (Transformation|SetWorldRotation (Variables|Default|GetWidget) "90.000000,0.000000,180.000000" false false)
  (UserInterface|SetWidget (Variables|Default|GetWidget) (stale EventBeginPlay _returnvalue))
  (Default|EventHealthEvent (stale EventBeginPlay _returnvalue) (Variables|Default|GetHealth) (Variables|Default|GetMaxHealth) (Variables|Default|GetGawainColour))
  (Default|EventStaminaEvent (stale EventBeginPlay _returnvalue) (Variables|Default|GetStamina) (Variables|Default|GetMaxStamina))
  (CallFunction|EventReplenishStamina))

(event EventCalculatePoints
  (params (Points :type Integer))
  ;[1 1 1] PointGain
  (Variables|Default|SetPoints (+ (Variables|Default|GetPoints) (* Points (Math|Float|Truncate (Variables|Default|GetMultiplier)))))
  (Variables|Default|SetMultiplier (+ (Variables|Default|GetMultiplier) 0.1)))

(event Input|GamepadEvents|GamepadRightTrigger
  (params (Key :type Key%20Structure :default "AnyKey"))
  (bind _realweapon (Variables|Default|GetRealWeapon))
  (bind _realweapon_2 (Variables|Default|GetRealWeapon))
  (bind _returnvalue (Actor|ActorHasTag _realweapon "RangedWeapon"))
  ;[1 1 1] RangedAttack
  (:Pressed
    (if _returnvalue
      (Variables|Default|SetIsRangedAttacking true)
      (bind _asacrossbow_bp (Utilities|Casting|CastToACrossbowBP _realweapon_2))
      (Default|PullTrigger _asacrossbow_bp)
      (Variables|Default|SetIsRangedAttacking false)
      (bind _returnvalue_2 (Class|GameplayStatics|GetPlayerControllerID))
      (Class|PlayerControllerID|IDTransfer(Message) _asacrossbow_bp _returnvalue_2)))
  (:Released
    (if _returnvalue
      (bind _asacrossbow_bp_2 (Utilities|Casting|CastToACrossbowBP _realweapon_2))
      (Default|ReleaseTrigger _asacrossbow_bp_2))))

(event Input|GamepadEvents|GamepadRightTrigger
  (params (Key :type Key%20Structure :default "AnyKey"))
  ;[1 1 1] Damages All Enemies In range
  (:Pressed
    (if (and (not (Variables|Default|GetIsAttacking)) (Actor|ActorHasTag (Variables|Default|GetRealWeapon) "MeleeWeapon"))
      (Variables|Default|SetIsAttacking true)
      (Audio|PlaySound2D "/Game/Audio/WeaponSFX/Weapon_Swing2.Weapon_Swing2"))))

(event Input|GamepadEvents|GamepadDPadLeft
  (params (Key :type Key%20Structure :default "AnyKey"))
  ;[1 1 1] Cheat/dev mode
)

(fn ConstructionScript
  (bind _foundwidgets (Widget|GetAllWidgetsOfClass "/Game/Blueprints/Menus/ArthurHUD.ArthurHUD_C" true))
  (for _array_element _foundwidgets
    (Variables|Default|SetPoints (Variables|/Game/Blueprints/Menus/ArthurHUD.ArthurHUD_C|GetPlayer3LastScore _array_element))
    (Variables|Default|SetHealth (Variables|Default|GetMaxHealth))
    (Variables|Default|SetStamina (Variables|Default|GetMaxStamina))
    (Variables|Default|SetMapArrowWidget (Variables|Default|GetP3MapArrow))))