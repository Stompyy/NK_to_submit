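; Parent player character Blueprint with twin-stick movement, a dash and a shove.
; Movement and Rotation macros apply dead zones and interpolation, facing the travel direction unless the right stick aims.
; Stamina gates the cooldown-limited dash and the shove, which messages overlapping ShoveAble actors.
; Events also handle stamina and health refill, being shoved, a map arrow and a warp-in area pulse, whose Slime knockback call is disconnected.
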(event Custom|Event%20SpawnKnockBack
  (bind _warpinaffectarea (Variables|Default|GetWarpInAffectArea))
  ;[1 1 1] Knock back enemies on self spawn in
  (for _array_element (Collision|GetOverlappingActors (Variables|Default|GetWarpInAffectArea) "/Game/Blueprints/Enemies/Slime.Slime_C" :!class /Script/Engine.PrimitiveComponent)
    _)
  (bind _affectareascale (Timeline|Warp%20in%20capsule%20growth PlayFromStart)
    (:Update
      (Transformation|SetWorldScale3D _warpinaffectarea (Math|Vector|MakeVector _affectareascale _affectareascale _affectareascale)))
    (:Finished
      (Transformation|SetWorldScale3D _warpinaffectarea "1.000000,1.000000,1.000000"))))

(event Custom|Event%20Replenish%20Health
  ;[1 1 1] For health pick up effect
  (Variables|Default|SetTempStartHealth (Variables|Default|GetHealth))
  (Variables|Default|SetTempDeltaHealth (- 1e+02 (Variables|Default|GetHealth)))
  (bind _health_replenish_rate (Timeline|HealthReplenish Play)
    (:Update
      (Variables|Default|SetHealth (+ (Variables|Default|GetTempStartHealth) (* _health_replenish_rate (Variables|Default|GetTempDeltaHealth)))))))

(event Custom|Event%20ShowMapArrow
  ;[1 1 1] When camera zooms out, show player position with an arrow
  (bind _returnvalue (UserInterface|CreateWidget (Variables|Default|GetMapArrowWidget)))
  (bind _asparent_map_widgets (Utilities|Casting|CastToParentMapWidgets _returnvalue))
  (Default|EventShowArrow _asparent_map_widgets)
  (UserInterface|Viewport|AddtoViewport _asparent_map_widgets 0))

(event Custom|Event%20Replenish%20Stamina
  ;[1 1 1] Stamina fills over time
  (if (< (Variables|Default|GetStamina) 99.0)
    (Variables|Default|SetStamina (+ (Variables|Default|GetStamina) (Variables|Default|GetStaminaReplenishRatePerFrame)))))

(event EventShoved
  (params (PositionOfPlayer :type Vector))
  ;[1 1 1] Apply Shove
  (Character|LaunchCharacter (* (- (Transformation|GetWorldLocation (Variables|Collision|GetCapsuleComponent)) PositionOfPlayer) (Variables|Default|GetPushPower)) false false))

(event Collision|EventActorBeginOverlap
  (params (OtherActor :type Actor%20Object%20Reference))
  ;[1 1 1] Adds and Removes enemies in range
  (if (Utilities|DoesObjectImplementInterface OtherActor "/Game/Blueprints/Interfaces/ShoveAble.ShoveAble_C")
    (Utilities|Array|Add (Variables|Default|GetShovablesInRange) OtherActor)))

(event Collision|EventActorEndOverlap
  (params (OtherActor :type Actor%20Object%20Reference))
  ;[1 1 1] Adds and Removes enemies in range
  (if (Utilities|DoesObjectImplementInterface OtherActor "/Game/Blueprints/Interfaces/ShoveAble.ShoveAble_C")
    (Utilities|Array|RemoveItem (Variables|Default|GetShovablesInRange) OtherActor)))

(event Input|AxisEvents|InputAxisMoveUp
  (params (AxisValue :type Float%20%28single-precision%29))
  (bind _isdead (Variables|Default|GetisDead))
  (bind _returnvalue (not _isdead))
  ;[1 1 1] Movement - aka Don't code late at night
  (bind _outputpin (Utilities|Movement _returnvalue _returnvalue _returnvalue AxisValue (stale Input|AxisEvents|InputAxisMoveRight AxisValue))))

(event Input|AxisEvents|InputAxisMoveRight
  (params (AxisValue :type Float%20%28single-precision%29))
  (bind _isdead (Variables|Default|GetisDead))
  (bind _returnvalue (not _isdead))
  ;[1 1 1] Movement - aka Don't code late at night
  (Utilities|Movement _returnvalue _returnvalue _returnvalue (stale Input|AxisEvents|InputAxisMoveUp AxisValue) AxisValue) ; enters at execute2
)

(event Input|AxisEvents|InputAxisLookup
  (params (AxisValue :type Float%20%28single-precision%29))
  ;[1 1 1] Rotation
  (Utilities|Rotation AxisValue (stale Input|AxisEvents|InputAxisLookRight AxisValue) (stale Input|AxisEvents|InputAxisMoveUp _outputpin)))

(event Input|AxisEvents|InputAxisLookRight
  (params (AxisValue :type Float%20%28single-precision%29))
  ;[1 1 1] Rotation
  (Utilities|Rotation (stale Input|AxisEvents|InputAxisLookup AxisValue) AxisValue (stale Input|AxisEvents|InputAxisMoveUp _outputpin)))

(event Input|GamepadEvents|GamepadFaceButtonRight
  (params (Key :type Key%20Structure :default "AnyKey"))
  ;[1 1 1] Dash
  (:Pressed
    (if (Math|Boolean|ANDBoolean (Variables|Default|GetCanDash) (not (Variables|Default|GetisDead)) (>= (Variables|Default|GetStamina) (Variables|Default|GetDashStaminaCost)))
      (Variables|Default|SetIsDashing false)
      (Variables|Default|SetStamina (- (Variables|Default|GetStamina) (Variables|Default|GetDashStaminaCost)))
      (Character|LaunchCharacter (* (Variables|Default|GetMovementVector) (Variables|Default|GetDashStrength)) false false)
      (Audio|PlaySound2D 0)
      (Variables|Default|SetCanDash false)
      (Utilities|FlowControl|Delay 2.0)
      (Variables|Default|SetIsDashing false)
      (Variables|Default|SetCanDash true))))

(event Input|GamepadEvents|GamepadLeftTrigger
  (params (Key :type Key%20Structure :default "AnyKey"))
  ;[1 1 1] LeftTrigger to Push Actors with Shovable in Range
  (:Pressed
    (if (>= (Variables|Default|GetStamina) (Variables|Default|GetShoveStaminaCost))
      (Variables|Default|SetStamina (- (Variables|Default|GetStamina) (Variables|Default|GetShoveStaminaCost)))
      (for _array_element (Variables|Default|GetShovablesInRange)
        (Class|ShoveAble|Shoved(Message) _array_element (Transformation|GetWorldLocation (Variables|Collision|GetCapsuleComponent)))))))

(event Input|GamepadEvents|GamepadDPadDown
  (params (Key :type Key%20Structure :default "AnyKey"))
  ;[1 1 1] debugs spawn follower
  (:Pressed
    (bind _outactors (Actor|GetAllActorsOfClass "/Game/Blueprints/ControllerBlueprints/SpawnFollower.SpawnFollower_C"))
    (for _array_element _outactors
      (Transformation|SetWorldLocation (Variables|Collision|GetCapsuleComponent) (Transformation|GetActorLocation _array_element) false true))))

(fn ConstructionScript)