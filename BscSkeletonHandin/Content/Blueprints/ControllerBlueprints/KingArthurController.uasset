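; Player controller for KingArthur that handles gamepad join/respawn and death, working with the NebulaKnights game mode to spawn and despawn players.
; Pressing Special Right spawns the player with identifying rumble and briefly blocks spawning on every KingArthurController to stagger spawns.
; Zero health deducts score, blocks respawn, and triggers a CameraUltimate death zoom unless the character fell, then destroys the weapon, despawns and restarts the shared spawn lockout.
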(event Custom|ControllerShake
  ;[1 1 1] Controller vibrate
  (Game|Feedback|PlayDynamicForceFeedback 0.5 (Variables|Default|GetSlowMoTimeDuration) true true true true))

(event Custom|Event%20DelaySpawn
  (params (DelayTime :type Float%20%28single-precision%29))
  ;[1 1 1] Sets all controllers as unable to spawn for a time, then sets as they can
  (bind _outactors (Actor|GetAllActorsOfClass "KingArthurController_C"))
  (for _array_element _outactors
    (Variables|KingArthurController_C|SetThisControllerAllowedToSpawn _array_element false))
  (Utilities|FlowControl|Delay DelayTime)
  (for _array_element_2 _outactors
    (Variables|KingArthurController_C|SetThisControllerAllowedToSpawn _array_element_2 true)))

(event EventTransferHealthInfo
  (params (Health :type Float%20%28single-precision%29) (PawnPosition :type Vector))
  (if (<= Health 0.0)
    (Variables|Default|SetisAlive false)
    ;[1 1 1] To allow death zoom in camera etc
    (Variables|Default|SetPlayerCanRespawn false)
    (bind _asnebula_knights (Utilities|Casting|CastToNebulaKnights (Game|GetGameMode)))
    (Variables|Default|SetScore (- (Variables|Default|GetScore) (Variables|Default|GetDeathScorePenalty)))
    (bind _asparent_character (Utilities|Casting|CastToParentCharacter (Pawn|GetControlledPawn)))
    (if (Variables|/Game/Blueprints/PlayerBlueprints/ParentCharacter.ParentCharacter_C|GetHasFallen _asparent_character)
      _
      (else
        (bind _ascamera_ultimate (Utilities|Casting|CastToCameraUltimate (Variables|Default|GetCameraUltimate)))
        (Variables|/Game/Blueprints/CameraRig/CameraUltimate.CameraUltimate_C|SetLastPlayerPosition _ascamera_ultimate PawnPosition)
        ;[1 1 1] Death event camera zoom in
        (bind _outactors (Actor|GetAllActorsOfClass "/Game/Blueprints/CameraRig/CameraUltimate.CameraUltimate_C"))
        (Default|EventZoomin (Utilities|Array|Get(acopy) _outactors))
        ;[1 1 1] For slow mo to have a player model in
        (Utilities|FlowControl|Delay 1.0)))
    (Actor|DestroyActor (Variables|/Game/Blueprints/PlayerBlueprints/ParentCharacter.ParentCharacter_C|GetRealWeapon _asparent_character))
    (Default|DespawnPlayer _asnebula_knights self)
    (CallFunction|EventDelaySpawn 2.0)))

(event Input|GamepadEvents|GamepadSpecialRight
  (params (Key :type Key%20Structure :default "AnyKey"))
  ;[1 1 1] If this controller spawns in, stop other players from spawning in for DelayTime
  (:Pressed
    (if (Variables|Default|GetThisControllerAllowedToSpawn)
      (CallFunction|EventDelaySpawn 0.5)
      ;[1 1 1] Basic bool checks
      (if (Variables|Default|GetPlayerCanRespawn)
        (if (not (Variables|Default|GetisAlive))
          (Variables|Default|SetisAlive true)
          ;[1 1 1] Spawns and assigns player in game mode
          (bind _outactors (Actor|GetAllActorsOfClass "/Game/Blueprints/NebulaKnights.NebulaKnights_C"))
          (Default|SpawnPlayers _outactors self)
          ;[1 1 1] Gives physical feedback at player spawn in to help player identify which character they are
          (Utilities|FlowControl|Delay (Variables|Default|GetSpawningAnimationDelay))
          (Game|Feedback|PlayDynamicForceFeedback 0.5 0.5 true true true true))))))

(fn ConstructionScript)