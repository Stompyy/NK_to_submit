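; Holy Grail pickup actor that awards points to the knight character who touches it.
; On overlap it casts to ParentCharacter, then tries King Arthur, Lancelot, Gawain and Percival in turn to call CalculatePoints with the prize value.
; It then destroys its Box component, and a timeline raises the mesh before destroying the actor.
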(event EventBeginPlay)

(event Collision|EventActorBeginOverlap
  (params (OtherActor :type Actor%20Object%20Reference))
  (bind _grailprizepoints (Variables|Default|GetGrailPrizePoints))
  ;[1 1 1] Pickup gives points to player
  (bind _asparent_character (Utilities|Casting|CastToParentCharacter OtherActor))
  (bind _asking_arthur (Utilities|Casting|CastToKingArthur _asparent_character)
    (:then
      (Default|CalculatePoints _asking_arthur _grailprizepoints))
    (:CastFailed
      (bind _assir_lancelot (Utilities|Casting|CastToSirLancelot _asparent_character)
        (:then
          (Default|CalculatePoints _assir_lancelot _grailprizepoints))
        (:CastFailed
          (bind _assir_gawain (Utilities|Casting|CastToSirGawain _asparent_character)
            (:then
              (Default|CalculatePoints _assir_gawain _grailprizepoints))
            (:CastFailed
              (bind _assir_percival (Utilities|Casting|CastToSirPercival _asparent_character))
              (Default|CalculatePoints _assir_percival _grailprizepoints)))))))
  (Components|DestroyComponent (Variables|Default|GetBox))
  ;[1 1 1] Grail rises then destroys itself
  (bind _grail_rise_amount (Timeline|GrailRise PlayFromStart)
    (:Update
      (Transformation|AddRelativeLocation (Variables|Default|GetStaticMesh) (Math|Vector|MakeVector 0.0 0.0 (* _grail_rise_amount (Variables|Default|GetFinalGrailHeightDisplacement))) false false))
    (:Finished
      (Actor|DestroyActor))))

(event EventTick
  (params (DeltaSeconds :type Float%20%28single-precision%29)))

(fn ConstructionScript)