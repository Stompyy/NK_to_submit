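; SpawnFollower is an AI character, apparently the players' moving respawn point, that trails the average-player-position actor.
; Each tick it issues AIMoveTo toward that actor, then checks for falling below a height limit.
; That check, kill-zone overlaps and an OverlappedKillZone event move it to the first living ParentCharacter, or to its starting location if no ParentCharacters exist.
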(event Custom|Event%20OverlappedKillZone
  ;[1 1 1] Every Killzone eventuality
  (bind _outactors (Actor|GetAllActorsOfClass "/Game/Blueprints/PlayerBlueprints/ParentCharacter.ParentCharacter_C"))
  (if (> (Utilities|Array|Length _outactors) 0)
    ;[1 1 1] Move to first valid players position it finds
    (bind _array_element (Utilities|Array|ForEachLoopwithBreak _outactors :!label _label)
      (:LoopBody
        (if (not (Variables|/Game/Blueprints/PlayerBlueprints/ParentCharacter.ParentCharacter_C|GetisDead _array_element))
          (Transformation|SetWorldLocation (Variables|Collision|GetCapsuleComponent) (Transformation|GetWorldLocation (Variables|/Script/Engine.Character|GetCapsuleComponent _array_element)) false false)
          (goto _label Break))))
    (else
      ;[1 1 1] Hard reset of position if no players available to spawn to
      (Transformation|SetWorldLocation (Variables|Collision|GetCapsuleComponent) (Variables|Default|GetOriginalLocation) false false))))

(event Custom|Event%20RespawnTheRespawner
  ;[1 1 1] Every Killzone eventuality
  (bind _outactors (Actor|GetAllActorsOfClass "/Game/Blueprints/PlayerBlueprints/ParentCharacter.ParentCharacter_C"))
  (if (> (Utilities|Array|Length _outactors) 0)
    ;[1 1 1] Move to first valid players position it finds
    (bind _array_element (Utilities|Array|ForEachLoopwithBreak _outactors :!label _label)
      (:LoopBody
        (if (not (Variables|/Game/Blueprints/PlayerBlueprints/ParentCharacter.ParentCharacter_C|GetisDead _array_element))
          (Transformation|SetWorldLocation (Variables|Collision|GetCapsuleComponent) (Transformation|GetWorldLocation (Variables|/Script/Engine.Character|GetCapsuleComponent _array_element)) false false)
          (goto _label Break))))
    (else
      ;[1 1 1] Hard reset of position if no players available to spawn to
      (Transformation|SetWorldLocation (Variables|Collision|GetCapsuleComponent) (Variables|Default|GetOriginalLocation) false false))))

(event EventBeginPlay
  (bind _outactors (Actor|GetAllActorsOfClass "/Game/Blueprints/CameraRig/AveragePositionOfPlayers_Blueprint.AveragePositionOfPlayers_Blueprint_C"))
  (Variables|Default|SetAveragePositionOfPlayers (Utilities|Array|Get(acopy) _outactors))
  ;[1 1 1] For a hard reset if needed
  (Variables|Default|SetOriginalLocation (Transformation|GetWorldLocation (Variables|Collision|GetCapsuleComponent))))

(event EventTick
  (params (DeltaSeconds :type Float%20%28single-precision%29))
  ;[1 1 1] AI follows players, avoiding holes, and falling platforms
  (AI|AIMoveTo self "0.000000, 0, 0" (Variables|Default|GetAveragePositionOfPlayers) 3e+02 false
    (:then
      (if (< (.z (Transformation|GetWorldLocation (Variables|Collision|GetCapsuleComponent))) -3e+03)
        (CallFunction|EventRespawntheRespawner)))))

(event Collision|EventActorBeginOverlap
  (params (OtherActor :type Actor%20Object%20Reference))
  ;[1 1 1] Every Killzone eventuality
  (Utilities|Casting|CastToKillZ OtherActor
    (:then
      _)
    (:CastFailed
      (Utilities|Casting|CastToKillZVolume OtherActor)))
  (bind _outactors (Actor|GetAllActorsOfClass "/Game/Blueprints/PlayerBlueprints/ParentCharacter.ParentCharacter_C"))
  (if (> (Utilities|Array|Length _outactors) 0)
    ;[1 1 1] Move to first valid players position it finds
    (bind _array_element (Utilities|Array|ForEachLoopwithBreak _outactors :!label _label)
      (:LoopBody
        (if (not (Variables|/Game/Blueprints/PlayerBlueprints/ParentCharacter.ParentCharacter_C|GetisDead _array_element))
          (Transformation|SetWorldLocation (Variables|Collision|GetCapsuleComponent) (Transformation|GetWorldLocation (Variables|/Script/Engine.Character|GetCapsuleComponent _array_element)) false false)
          (goto _label Break))))
    (else
      ;[1 1 1] Hard reset of position if no players available to spawn to
      (Transformation|SetWorldLocation (Variables|Collision|GetCapsuleComponent) (Variables|Default|GetOriginalLocation) false false))))

(fn ConstructionScript
  ;[1 1 1] Sets movement speed
  (Variables|/Script/Engine.CharacterMovementComponent|SetMaxWalkSpeed (Variables|Character|GetCharacterMovement) 1e+03))