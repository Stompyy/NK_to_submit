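; HealthPickup is a pickup that restores health to a ParentCharacter that touches it.
; Each tick it yaws its static mesh by a small random amount.
; On BoxTrigger overlap by a ParentCharacter it plays the collection sound, then, if Health is below a near-full threshold, calls the character's EventReplenishHealth and destroys itself.
; The sound plays even when the character is too healthy to consume the pickup.
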(event OnComponentBeginOverlap(BoxTrigger)
  (params (OverlappedComponent :type Primitive%20Component%20Object%20Reference) (OtherActor :type Actor%20Object%20Reference) (OtherComp :type Primitive%20Component%20Object%20Reference) (OtherBodyIndex :type Integer) (bFromSweep :type Boolean) (SweepResult :type Hit%20Result%20Structure%20%28by%20ref%29))
  (bind _asparent_character (Utilities|Casting|CastToParentCharacter OtherActor))
  (Audio|PlaySound2D "/Game/Audio/PickupSFX/Health_Pack_Collected.Health_Pack_Collected")
  (if (not (>= (Variables|/Game/Blueprints/PlayerBlueprints/ParentCharacter.ParentCharacter_C|GetHealth _asparent_character) 99.0))
    (Default|EventReplenishHealth _asparent_character)
    (Actor|DestroyActor)))

(event EventBeginPlay)

(event Collision|EventActorBeginOverlap
  (params (OtherActor :type Actor%20Object%20Reference)))

(event EventTick
  (params (DeltaSeconds :type Float%20%28single-precision%29))
  (Transformation|AddWorldRotation (Variables|Default|GetStaticMesh) (Math|Rotator|MakeRotator 0.0 0.0 (* (Math|Random|RandomFloat) 2.0)) false false))

(fn ConstructionScript)