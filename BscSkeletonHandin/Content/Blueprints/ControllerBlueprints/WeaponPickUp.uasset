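; Weapon pickup actor that hands a randomly selected weapon to the overlapping character, then destroys itself.
; BeginPlay picks from ChosenWeapons with RandomInteger(Length - 1), whose exclusive bound leaves out the last entry.
; Box overlap casts to ParentCharacter and passes the weapon through PickupTypeMessage.
; The construction script randomizes a three-axis spin per instance, which Tick applies to the mesh without delta-time scaling.
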(event OnComponentBeginOverlap(Box)
  (params (OverlappedComponent :type Primitive%20Component%20Object%20Reference) (OtherActor :type Actor%20Object%20Reference) (OtherComp :type Primitive%20Component%20Object%20Reference) (OtherBodyIndex :type Integer) (bFromSweep :type Boolean) (SweepResult :type Hit%20Result%20Structure%20%28by%20ref%29))
  ;[1 1 1] On overlap, if player, assign them this pickup's specific weapon, and destroy self
  (bind _asparent_character (Utilities|Casting|CastToParentCharacter OtherActor))
  (Class|Pick2player|PickupType(Message) _asparent_character (Variables|Default|GetChosenWeapon))
  (Actor|DestroyActor))

(event EventBeginPlay
  (bind _chosenweapons (Variables|Default|GetChosenWeapons))
  ;[1 1 1] Choose random weapon from list
  (Variables|Default|SetChosenWeapon (Utilities|Array|Get(acopy) _chosenweapons (Math|Random|RandomInteger (- (Utilities|Array|Length _chosenweapons) 1)))))

(event EventTick
  (params (DeltaSeconds :type Float%20%28single-precision%29))
  ;[1 1 1] Rotate on tick
  (Transformation|AddWorldRotation (Variables|Default|GetStaticMesh) (Math|Rotator|MakeRotator (Variables|Default|GetRandomXaxisSpin) (Variables|Default|GetRandomYaxisSpin) (Variables|Default|GetRandomZaxisSpin)) false false))

(fn ConstructionScript
  ;[1 1 1] Sets an individual random spin to every pick up
  (Variables|Default|SetRandomXaxisSpin (Math|Random|RandomFloatinRange -2.0 2.0))
  (Variables|Default|SetRandomYaxisSpin (Math|Random|RandomFloatinRange -2.0 2.0))
  (Variables|Default|SetRandomZaxisSpin (Math|Random|RandomFloatinRange -2.0 2.0)))