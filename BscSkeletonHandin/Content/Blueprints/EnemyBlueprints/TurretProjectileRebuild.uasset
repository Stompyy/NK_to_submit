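; Turret projectile Blueprint that explodes on contact, breaking destructible wall segments or damaging tagged player targets.
; Overlap and Hit events share one cast check: walls receive radial damage, then are destroyed after a delay.
; Other actors, except those tagged Door, trigger the explosion, with player-tagged ones first receiving a health-change message.
; Non-wall impacts remove the mesh and root to halt the effect, then destroy the projectile after the particle delay.
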(event Collision|EventActorBeginOverlap
  (params (OtherActor :type Actor%20Object%20Reference))
  ;[1 1 1] Currently only overlap is generating events.
  ;[1 1 1] 'If' statement for is destructable wall
  (bind _asdestructable_wall_segment_bp (Utilities|Casting|CastToDestructableWallSegment_BP OtherActor)
    (:then
      (Components|Activation|Activate (Variables|Default|GetExplosion) false)
      ;[1 1 1] Destroy Destructable actor
      (Game|Damage|ApplyRadialDamage 1e+03 (Transformation|GetWorldLocation (Variables|Default|GetMesh)) 1e+03 "/Script/Engine.DamageType" 0 0 0 true "ECC_Visibility")
      (Components|DestroyComponent (Variables|Default|GetDefaultSceneRoot))
      ;[1 1 1] Connect to destroy destructable wall actor after hit
      (Utilities|FlowControl|Delay 2.0)
      (Actor|DestroyActor _asdestructable_wall_segment_bp))
    (:CastFailed
      (if (not (Actor|ActorHasTag OtherActor "Door"))
        (if (Actor|ActorHasTag OtherActor (Variables|Default|GetPlayerTagForBullets))
          (Class|IDamageable|Affecthealth(Message) OtherActor (Variables|Default|GetweaponDamage)))
        (Components|Activation|Activate (Variables|Default|GetExplosion) false)
        (Components|DestroyComponent (Variables|Default|GetMesh))
        ;[1 1 1] If Default scene root is being destroyed in previous function, then this bit is not necessary
        (Utilities|FlowControl|Delay (Variables|Default|GetTimeForParticleEffect))
        (Actor|DestroyActor)))))

(event Collision|EventHit
  (params (MyComp :type Primitive%20Component%20Object%20Reference) (Other :type Actor%20Object%20Reference) (OtherComp :type Primitive%20Component%20Object%20Reference) (bSelfMoved :type Boolean) (HitLocation :type Vector :default "0, 0, 0") (HitNormal :type Vector :default "0, 0, 0") (NormalImpulse :type Vector :default "0, 0, 0") (Hit :type Hit%20Result%20Structure%20%28by%20ref%29))
  ;[1 1 1] Would be better for destructablecomponant hit as it provides a precise hit location
  ;[1 1 1] 'If' statement for is destructable wall
  (bind _asdestructable_wall_segment_bp (Utilities|Casting|CastToDestructableWallSegment_BP (stale Collision|EventActorBeginOverlap OtherActor))
    (:then
      (Components|Activation|Activate (Variables|Default|GetExplosion) false)
      ;[1 1 1] Destroy Destructable actor
      (Game|Damage|ApplyRadialDamage 1e+03 (Transformation|GetWorldLocation (Variables|Default|GetMesh)) 1e+03 "/Script/Engine.DamageType" 0 0 0 true "ECC_Visibility")
      (Components|DestroyComponent (Variables|Default|GetDefaultSceneRoot))
      ;[1 1 1] Connect to destroy destructable wall actor after hit
      (Utilities|FlowControl|Delay 2.0)
      (Actor|DestroyActor _asdestructable_wall_segment_bp))
    (:CastFailed
      (if (not (Actor|ActorHasTag (stale Collision|EventActorBeginOverlap OtherActor) "Door"))
        (if (Actor|ActorHasTag (stale Collision|EventActorBeginOverlap OtherActor) (Variables|Default|GetPlayerTagForBullets))
          (Class|IDamageable|Affecthealth(Message) (stale Collision|EventActorBeginOverlap OtherActor) (Variables|Default|GetweaponDamage)))
        (Components|Activation|Activate (Variables|Default|GetExplosion) false)
        (Components|DestroyComponent (Variables|Default|GetMesh))
        ;[1 1 1] If Default scene root is being destroyed in previous function, then this bit is not necessary
        (Utilities|FlowControl|Delay (Variables|Default|GetTimeForParticleEffect))
        (Actor|DestroyActor)))))

(fn ConstructionScript)