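; Hidden enemy turret that slides open its cover and rises from the floor when a player enters its trigger box.
; While players remain, Tick finds the nearest, yaw-lerps toward them and fires delayed three-projectile bursts; otherwise it spins idly.
; Crossbow hits award owner points and destroy it, melee hits only award points, and health loss can also kill it.
; Death triggers explosion and radial damage, then timelines lower it and seal the floor.
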(event OnComponentBeginOverlap(Capsule)
  (params (OverlappedComponent :type Primitive%20Component%20Object%20Reference) (OtherActor :type Actor%20Object%20Reference) (OtherComp :type Primitive%20Component%20Object%20Reference) (OtherBodyIndex :type Integer) (bFromSweep :type Boolean) (SweepResult :type Hit%20Result%20Structure%20%28by%20ref%29))
  (bind _turretkillpoints (Variables|Default|GetTurretKillPoints))
  ;[1 1 1] Allows player to destroy turret with weapon attack, and increases score for doing so
  ;;[1 1 1] Melee weapon
  (bind _asmelee_weapon (Utilities|Casting|CastToMeleeWeapon OtherActor)
    (:then
      (if (Variables|/Game/Blueprints/Weapons/MeleeWeapon.MeleeWeapon_C|GetCanAttack _asmelee_weapon)
        (bind _aspawn (Utilities|GetPlayerKilling _asmelee_weapon)
          (:OutputPin
            (Class|PointGain|CalculatePoints(Message) _aspawn (Variables|Default|GetTurretKillPoints))))))
    (:CastFailed
      ;;[1 1 1] Crossbow projectile
      (bind _ascrossbow_projectile (Utilities|Casting|CastToCrossbowProjectile OtherActor))
      (bind _asking_arthur (Utilities|Casting|CastToKingArthur (Components|GetOwner _ascrossbow_projectile))
        (:then
          (Default|CalculatePoints _asking_arthur _turretkillpoints))
        (:CastFailed
          (bind _assir_lancelot (Utilities|Casting|CastToSirLancelot (Components|GetOwner _ascrossbow_projectile))
            (:then
              (Default|CalculatePoints _assir_lancelot _turretkillpoints))
            (:CastFailed
              (bind _assir_gawain (Utilities|Casting|CastToSirGawain (Components|GetOwner _ascrossbow_projectile))
                (:then
                  (Default|CalculatePoints _assir_gawain _turretkillpoints))
                (:CastFailed
                  (bind _assir_percival (Utilities|Casting|CastToSirPercival (Components|GetOwner _ascrossbow_projectile)))
                  (Default|CalculatePoints _assir_percival _turretkillpoints)))))))
      (CallFunction|EventTurretDeath))))

(event OnComponentBeginOverlap(Box)
  (params (OverlappedComponent :type Primitive%20Component%20Object%20Reference) (OtherActor :type Actor%20Object%20Reference) (OtherComp :type Primitive%20Component%20Object%20Reference) (OtherBodyIndex :type Integer) (bFromSweep :type Boolean) (SweepResult :type Hit%20Result%20Structure%20%28by%20ref%29))
  ;[1 1 1] Triggers on proximity (Enter box)
  (Utilities|Casting|CastToParentCharacter OtherActor)
  (Math|Integer|IncrementInt (Variables|Default|GetnumberOfPlayersInBox)
    (:%20%20
      (if (Variables|Default|Getemerged)
        (Variables|Default|SetunleashHell true)
        (else
          (CallFunction|EmergeTurret)
          (Variables|Default|Setemerged true))))))

(event OnComponentEndOverlap(Box)
  (params (OverlappedComponent :type Primitive%20Component%20Object%20Reference) (OtherActor :type Actor%20Object%20Reference) (OtherComp :type Primitive%20Component%20Object%20Reference) (OtherBodyIndex :type Integer))
  ;[1 1 1] Triggers on proximity (Enter box)
  (Utilities|Casting|CastToParentCharacter OtherActor)
  (Math|Integer|DecrementInt (Variables|Default|GetnumberOfPlayersInBox)
    (:%20%20
      (if (== (Variables|Default|GetnumberOfPlayersInBox) 0)
        (Variables|Default|SetunleashHell false)))))

(event Custom|FireBullet
  (bind _firedirection (Variables|Default|GetfireDirection))
  (bind _returnvalue (Transformation|GetWorldTransform _firedirection))
  ;[1 1 1] Fire weapon and instantiate bullet
  (if (Variables|Default|GetIsValidTarget)
    ;;[1 1 1] Collapse into looping function?
    (Game|SpawnActorfromClass "/Game/Blueprints/EnemyBlueprints/TurretProjectileRebuild.TurretProjectileRebuild_C" _returnvalue "Undefined" 0 0)
    (Audio|Components|Audio|Play (Variables|Default|GetGunShot) 0.0)
    (Utilities|FlowControl|Delay 0.1)
    (Game|SpawnActorfromClass "/Game/Blueprints/EnemyBlueprints/TurretProjectileRebuild.TurretProjectileRebuild_C" _returnvalue "Undefined" 0 0)
    (Utilities|FlowControl|Delay 0.1)
    (Game|SpawnActorfromClass "/Game/Blueprints/EnemyBlueprints/TurretProjectileRebuild.TurretProjectileRebuild_C" _returnvalue "Undefined" 0 0)
    (Audio|Components|Audio|Play (Variables|Default|GetGunShot) 0.0)
    (CallFunction|FireMuzzleAnim)
    (Utilities|FlowControl|Delay (/ 1.0 (Variables|Default|GetFireRate)))
    (Variables|Default|SetfireDelayFinished true)))

(event Custom|EmergeTurret
  ;[1 1 1] Emerge Turret
  (Utilities|FlowControl|DoOnce false
    (:Completed
      (CallFunction|EmergeTurretAnimation))))

(event Custom|EmergeTurretAnimation
  ;[1 1 1] Emerge turret event
  ;;[1 1 1] Slide back cover
  (bind _newtrack_0 (Timeline|slideBackTop PlayFromStart)
    (:Update
      (Transformation|SetRelativeLocation (Variables|Default|Getcover) (Math|Vector|MakeVector _newtrack_0 0.0 0.0) false false))
    (:Finished
      (Components|DestroyComponent (Variables|Default|Getcover))
      ;;[1 1 1] Raise turret out of ground
      (bind _turretheight (Timeline|raiseTurret PlayFromStart)
        (:Update
          (Transformation|SetRelativeLocation (Variables|Default|GetBase) (Math|Vector|MakeVector 0.0 0.0 _turretheight) false false))
        (:Finished
          (Components|DestroyComponent (Variables|Default|GetundergroundBox))
          (Variables|Default|Setemerged true))))))

(event Custom|FireMuzzleAnim
  ;[1 1 1] Muzzle fire animation
  (bind _newtrack_0 (Timeline|muzzleFireMovement PlayFromStart)
    (:Update
      (Transformation|SetRelativeLocation (Variables|Default|GetMuzzle) (Math|Vector|MakeVector _newtrack_0 0.0 0.0) false false))))

(event Custom|Event%20TurretDeath
  (bind _explosion (Variables|Default|GetExplosion))
  (Utilities|FlowControl|DoOnce false
    (:Completed
      ;[1 1 1] Destroys destructible elements and activates particle effects
      (Variables|Default|SetTurretDied true)
      (Components|DestroyComponent (Variables|Default|GetMuzzle))
      (Components|Activation|Activate _explosion false)
      (Audio|Components|Audio|Play (Variables|Default|GetExplode) 0.0)
      (Game|Damage|ApplyRadialDamage 1e+03 (Transformation|GetWorldLocation _explosion) 1e+01 0 0 0 0 false "ECC_Visibility")
      (Components|Activation|Activate (Variables|Default|GetSparks) false)
      (Utilities|FlowControl|Delay 1.0)
      ;[1 1 1] Seperates floor piece from the actor
      (Transformation|DetachFromComponent (Variables|Default|GetNewBase) "KeepWorld" "KeepWorld" "KeepWorld" true)
      ;[1 1 1] Animates turret lowering and floor piece moving over hole
      (bind _turretheight (Timeline|Hide%20Turret ReverseFromEnd)
        (:Update
          (Transformation|SetRelativeLocation (Variables|Default|GetBase) (Math|Vector|MakeVector 0.0 0.0 _turretheight) false false))
        (:Finished
          (bind _turretheight_2 (Timeline|Timeline_0 PlayFromStart)
            (:Update
              (Transformation|SetRelativeLocation (Variables|Default|GetNewBaseMiddle) (Math|Vector|MakeVector 0.0 0.0 _turretheight_2) false false))
            (:Finished
              ;[1 1 1] Deletes everything that is not now part of the floor
              (Components|DestroyComponent (Variables|Default|GetSparks)))))))))

(event Custom|FindClosestPlayer
  ;[1 1 1] New version of find closest player
  (bind _outactors (Actor|GetAllActorsOfClass "/Game/Blueprints/PlayerBlueprints/ParentCharacter.ParentCharacter_C"))
  (for _array_element _outactors
    (if (< (Transformation|GetDistanceTo _array_element) (Variables|Default|GetcurrentMinDistance))
      (Variables|Default|SetclosestPlayer _array_element)
      (Variables|Default|SetcurrentMinDistance (Transformation|GetDistanceTo _array_element))))
  (Variables|Default|SetcurrentMinDistance 99999999.0))

(event Custom|getLookAtRotation
  (bind _turnlerp (Variables|Default|GetturnLerp))
  (bind _closestplayer (Variables|Default|GetclosestPlayer))
  (bind _top_dm (Variables|Default|GetTop_DM))
  (bind _top_dm_2 (Variables|Default|GetTop_DM))
  (bind _returnvalue (Transformation|GetWorldRotation _top_dm))
  (bind _returnvalue_2 (VehicleSound|GetRootComponent _closestplayer))
  (bind _returnvalue_3 (Transformation|GetWorldLocation _top_dm_2))
  (bind _returnvalue_4 (Transformation|GetWorldLocation _returnvalue_2))
  (bind _returnvalue_5 (Math|Rotator|FindLookatRotation _returnvalue_3 _returnvalue_4))
  (bind _returnvalue_6 (Math|Rotator|Lerp(Rotator) _returnvalue _returnvalue_5 _turnlerp true))
  (bind _yaw (Math|Rotator|BreakRotator _returnvalue_6))
  ;[1 1 1] Lerp current turret rotation to target rotation
  (Variables|Default|SettargetPlayerAngle (Math|Rotator|MakeRotator 0.0 0.0 _yaw))
  (Variables|Default|SettargetPlayerAngleZ _yaw))

(event EventTick
  (params (DeltaSeconds :type Float%20%28single-precision%29))
  (bind _targetplayeranglez (Variables|Default|GettargetPlayerAngleZ))
  ;[1 1 1] Event Tick
  (if (not (Variables|Default|GetTurretDied))
    (if (Variables|Default|GetunleashHell)
      (CallFunction|FindClosestPlayer)
      (CallFunction|GetLookatRotation)
      ;[1 1 1] Calls firing function to instantiate bullet
      (if (or (>= _targetplayeranglez (Variables|Default|GetminFireAtAngle)) (<= _targetplayeranglez (Variables|Default|GetmaxFireAtAngle)))
        (if (Variables|Default|GetfireDelayFinished)
          (Variables|Default|SetfireDelayFinished false)
          (CallFunction|FireBullet)))
      ;[1 1 1] Aim at player
      (Transformation|SetWorldRotation (Variables|Default|GetTop_DM) (Variables|Default|GettargetPlayerAngle) false false)
      ;[1 1 1] If not aiming directly at player (turnLerp == 1) then increment (turnLerp += speed)
      (if (>= (Variables|Default|GetturnLerp) 1.0)
        (Variables|Default|SetturnLerp 1.0)
        (else
          (Variables|Default|SetturnLerp (+ (Variables|Default|GetturnLerp) (Variables|Default|GetaimingTurnSpeed)))))
      (else
        ;[1 1 1] Rotate turret when player not near and reset lerp variable
        (Transformation|AddLocalRotation (Variables|Default|GetTop_DM) (Math|Rotator|MakeRotator 0.0 0.0 (Variables|Default|GetturretRotSpeed)) false false)
        (Variables|Default|SetturnLerp 0.0)))))

(event EventBeginPlay)

(event EventAffecthealth
  (params (DeltaDamage :type Float%20%28single-precision%29) (Player :type Actor%20Object%20Reference))
  ;[1 1 1] Should we use a health float or keep it one hit kill on overlap event?
  (bind _output_get (Variables|Default|SetHealth (- (Variables|Default|GetHealth) DeltaDamage)))
  (if (<= _output_get 0.0)
    (CallFunction|EventTurretDeath)))

(fn ConstructionScript
  (Transformation|SetWorldScale3D (Variables|Default|GetBox) (Variables|Default|GetTriggerBoxSize)))