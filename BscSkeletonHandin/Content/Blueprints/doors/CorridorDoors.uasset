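; Sliding corridor double door that opens once every ParentCharacter gathers in the front trigger, then moves again when all gather in the back trigger, normally closing for good.
; Overlap events track characters per trigger and compare counts against all ParentCharacter actors in the level.
; Tick offsets both leaves by a fixed step, reversing direction after opening.
; A spawned ArchLightBP changes colour whenever a movement completes.
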(event OnComponentBeginOverlap(FrontCheck)
  (params (OverlappedComponent :type Primitive%20Component%20Object%20Reference) (OtherActor :type Actor%20Object%20Reference) (OtherComp :type Primitive%20Component%20Object%20Reference) (OtherBodyIndex :type Integer) (bFromSweep :type Boolean) (SweepResult :type Hit%20Result%20Structure%20%28by%20ref%29))
  (bind _playerrefarray (Variables|Default|GetPlayerRefArray))
  (bind _asparent_character (Utilities|Casting|CastToParentCharacter OtherActor))
  (Utilities|Array|AddUnique _playerrefarray _asparent_character)
  (bind _outactors (Actor|GetAllActorsOfClass "/Game/Blueprints/PlayerBlueprints/ParentCharacter.ParentCharacter_C"))
  (if (== (Utilities|Array|Length _outactors) (Utilities|Array|Length _playerrefarray))
    (if (not (Variables|Default|GetDoorsAreOpen))
      (Variables|Default|SetOpenDoors true))))

(event OnComponentBeginOverlap(BackCheck)
  (params (OverlappedComponent :type Primitive%20Component%20Object%20Reference) (OtherActor :type Actor%20Object%20Reference) (OtherComp :type Primitive%20Component%20Object%20Reference) (OtherBodyIndex :type Integer) (bFromSweep :type Boolean) (SweepResult :type Hit%20Result%20Structure%20%28by%20ref%29))
  (bind _playerrefarrayclose (Variables|Default|GetPlayerRefArrayClose))
  (bind _asparent_character (Utilities|Casting|CastToParentCharacter OtherActor))
  (Utilities|Array|AddUnique _playerrefarrayclose _asparent_character)
  (bind _outactors (Actor|GetAllActorsOfClass "/Game/Blueprints/PlayerBlueprints/ParentCharacter.ParentCharacter_C"))
  (if (== (Utilities|Array|Length _outactors) (Utilities|Array|Length _playerrefarrayclose))
    (if (not (Variables|Default|GetOpenDoors))
      (Variables|Default|SetDoneWithThisDoor true)
      (Variables|Default|SetOpenDoors true))))

(event OnComponentEndOverlap(FrontCheck)
  (params (OverlappedComponent :type Primitive%20Component%20Object%20Reference) (OtherActor :type Actor%20Object%20Reference) (OtherComp :type Primitive%20Component%20Object%20Reference) (OtherBodyIndex :type Integer))
  (bind _asparent_character (Utilities|Casting|CastToParentCharacter OtherActor))
  (Utilities|Array|RemoveItem (Variables|Default|GetPlayerRefArray) _asparent_character))

(event OnComponentEndOverlap(BackCheck)
  (params (OverlappedComponent :type Primitive%20Component%20Object%20Reference) (OtherActor :type Actor%20Object%20Reference) (OtherComp :type Primitive%20Component%20Object%20Reference) (OtherBodyIndex :type Integer))
  (bind _asparent_character (Utilities|Casting|CastToParentCharacter OtherActor))
  (Utilities|Array|RemoveItem (Variables|Default|GetPlayerRefArrayClose) _asparent_character))

(event EventBeginPlay
  (bind _returnvalue (Game|SpawnActorfromClass "/Game/Blueprints/doors/ArchLightBP.ArchLightBP_C" (Transformation|GetWorldTransform (Variables|Default|GetScene)) "Undefined" 0 0))
  (Variables|Default|SetArchLight _returnvalue))

(event EventTick
  (params (DeltaSeconds :type Float%20%28single-precision%29))
  (if (not (Variables|Default|GetFinished))
    (if (Variables|Default|GetOpenDoors)
      (Audio|Components|Audio|Play (Variables|Default|GetDoors) 0.0)
      (Transformation|AddLocalOffset (Variables|Default|GetRightDoor) (Math|Vector|MakeVector 0.0 (* (Variables|Default|GetOffsetPerTick) (Variables|Default|GetLeftDoorDirection)) 0.0) false false)
      (Transformation|AddLocalOffset (Variables|Default|GetLeftDoor) (Math|Vector|MakeVector 0.0 (* (Variables|Default|GetOffsetPerTick) (Variables|Default|GetRightDoorDirection)) 0.0) false false)
      (Variables|Default|SetDistanceMoved (+ (Variables|Default|GetDistanceMoved) (Variables|Default|GetOffsetPerTick)))
      (if (<= (Variables|Default|GetDistanceToMove) (Variables|Default|GetDistanceMoved))
        (Default|EventChangeColour (Variables|Default|GetArchLight))
        (if (Variables|Default|GetDoneWithThisDoor)
          (Variables|Default|SetFinished true)
          (else
            (Variables|Default|SetOpenDoors false)
            (Variables|Default|SetDoorsAreOpen true)
            (Variables|Default|SetLeftDoorDirection 1.0)
            (Variables|Default|SetRightDoorDirection -1.0)
            (Variables|Default|SetDistanceMoved 0.0)))))))

(fn ConstructionScript
  (Class|SceneComponent|AddLocalTransform (Variables|Default|GetFrontCheck) (Variables|Default|GetFrontCheckTransform) false false)
  (Class|SceneComponent|AddLocalTransform (Variables|Default|GetBackCheck) (Variables|Default|GetBackCheckTransform) false false))