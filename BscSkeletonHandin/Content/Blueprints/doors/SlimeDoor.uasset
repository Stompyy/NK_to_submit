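; SlimeDoor is a double door that opens once enough slimes die after the player has entered its room.
; An overlap collider, resized in construction, flags player entry, enabling EnemyDeadCheck to count kills toward the required total.
; Tick then slides both doors apart until maximum offset, repeatedly calling the colour change on an arch light spawned at BeginPlay.
; The CheckIfRightDoorAndOpen graph compares against an array minimum but performs no action.
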(event OnComponentBeginOverlap(PlayerInRoomCollider)
  (params (OverlappedComponent :type Primitive%20Component%20Object%20Reference) (OtherActor :type Actor%20Object%20Reference) (OtherComp :type Primitive%20Component%20Object%20Reference) (OtherBodyIndex :type Integer) (bFromSweep :type Boolean) (SweepResult :type Hit%20Result%20Structure%20%28by%20ref%29))
  ;[1 1 1] Checks if the player has entered the room if so set bool to true
  (Utilities|Casting|CastToParentCharacter OtherActor)
  (Variables|Default|SetPlayerEnteredRoom true))

(event Custom|EnemyDeadCheck
  ;[1 1 1] EnemyDead Check is called everytime a slime dies in a room with a slime door. When the required kills are made the doors open
  (if (Variables|Default|GetPlayerEnteredRoom)
    (bind _result (Math|Integer|IncrementInt (Variables|Default|GetDeadEnemiesDoor))
      (:%20%20
        (if (>= _result (Variables|Default|GetRequiredKillsToOpen))
          (Variables|Default|SetOpenDoors true)
          (else
            (Variables|Default|SetOpenDoors false)))))))

(event EventBeginPlay
  ;[1 1 1] Spawns Archlight in the location of the Light actor. On begin play.
  (bind _returnvalue (Game|SpawnActorfromClass "/Game/Blueprints/doors/ArchLightBP.ArchLightBP_C" (Transformation|GetWorldTransform (Variables|Default|GetLight)) "AlwaysSpawn" 0 0))
  (Variables|Default|SetArchLight _returnvalue))

(event EventTick
  (params (DeltaSeconds :type Float%20%28single-precision%29))
  (if (Variables|Default|GetOpenDoors)
    (if (not (Variables|Default|GetDoorsOpen))
      ;[1 1 1] Adds Offset to right door to open it
      (Transformation|AddLocalOffset (Variables|Default|GetRightDoor) (Math|Vector|MakeVector 0.0 (* (Variables|Default|GetOffsetPerTick) -1.0) 0.0) false false)
      ;[1 1 1] Adds Offset To left door to open it
      (Transformation|AddLocalOffset (Variables|Default|GetLeftDoor) (Math|Vector|MakeVector 0.0 (Variables|Default|GetOffsetPerTick) 0.0) false false)
      ;[1 1 1] Sets the bool doors open to be true when they opened completely. The event to turn the Arch light green is also called here
      (Variables|Default|SetDistanceMoved (+ (Variables|Default|GetDistanceMoved) (Variables|Default|GetOffsetPerTick)))
      (Variables|Default|SetDoorsOpen (<= (Variables|Default|GetMaxOffset) (Variables|Default|GetDistanceMoved)))
      (Default|EventChangeColour (Variables|Default|GetArchLight)))))

(fn ConstructionScript
  (Class|SceneComponent|AddLocalTransform (Variables|Default|GetPlayerInRoomCollider) (Math|Transform|MakeTransform "0, 0, 0" "0, 0, 0" (Variables|Default|GetSizeOfBox)) false false))